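; Example navigation UI Blueprint that draws a guide path from the player to the nearest objective actor, such as a victim in the fire scenario.
; BeginPlay gathers objectives by class and starts a looping timer that refreshes the path every quarter second.
; Each refresh picks the objective with the shortest navmesh path length, rebuilds a linear spline slightly above the floor along that path, and recreates spline mesh segments between its points.
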(event `self.ReceiveBeginPlay`
  (`|ExecutionSequence`
    (:`then_0`
      ;[0 0 0] Use "Get All Actors of Class" to get an array containing the objectives (in the case of fire scenario, the two victims placed in the level)
      (bind _outactors (`GameplayStatics.GetAllActorsOfClass` (`self.ObjectiveClass`)))
      (set `self.ObjectiveArray` _outactors))
    (:`then_1`
      (`KismetSystemLibrary.K2_SetTimerDelegate` (delegate `UpdatePath`) 0.25 true) ; Executing this node once on BeginPlay, will cause it to execute\nthe connected event, UpdatePath, once every 0.25 seconds\ncontinuously on a loop
    )))

(event `UpdatePath`
  ;[0 0 0] Only run this functionality if our "Get All Actors of Class" actually found some actors, and populated ObjectiveArray with them. Otherwise, we would be trying to draw a path to something that doesn't exist
  (if (> (`KismetArrayLibrary.Array_Length` (`self.ObjectiveArray`)) 0)
    (`|ExecutionSequence`
      (:`then_0`
        ;[0 0 0] Clear the spline points of PathSpline and remove all the spline meshes in PathSplineMeshArray from the last update
        (`SplineComponent.ClearSplinePoints` (`self.PathSpline`) true)
        (`ActorComponent.K2_DestroyComponent` (`self.PathSplineMeshArray`))
        (`KismetArrayLibrary.Array_Clear` (`self.PathSplineMeshArray`)))
      (:`then_1`
        (bind _outclosestobjective (`self.FindClosestObjective`))
        ;[0 0 0] Calculate a path from the player to the closest objective
        (bind _returnvalue (`NavigationSystemV1.FindPathToLocationSynchronously` (`self.K2_GetActorLocation` (`GameplayStatics.GetPlayerPawn` 0)) (`self.K2_GetActorLocation` _outclosestobjective) null null))
        ;[0 0 0] For each point along the path, add a point to PathSpline, so that the shape of PathSpline matches that of the path
        (for (_array_element _array_index) (`NavigationPath.PathPoints` _returnvalue)
          (`SplineComponent.AddSplinePoint` (`self.PathSpline`) (+ (0.0 0.0 20.0) _array_element) "World" true)
          (`SplineComponent.SetSplinePointType` (`self.PathSpline`) _array_index "Linear" true) ; Set the spline point type to be linear so that it\nforms straight lines rather than wide curves
        ))
      (:`then_2`
        ;[0 0 0] Now that PathSpline has been arranged to match our path, we can add a spline mesh between each point on PathSpline, and manipulate it to render along the spline
        (for _index (range (+ (- (`SplineComponent.GetNumberOfSplinePoints` (`self.PathSpline`)) 2) 1))
          (bind _returnvalue_2 (`AddComponent|NODE_AddSplineMeshComponent-0` :`bManualAttachment` true)) ; Add a new mesh that will be rendered between the points on the spline
          (`KismetArrayLibrary.Array_Add` (`self.PathSplineMeshArray`) _returnvalue_2)
          (`SplineMeshComponent.SetStartAndEnd` _returnvalue_2 (`SplineComponent.GetLocationAndTangentAtSplinePoint` (`self.PathSpline`) _index "World") (0.0 0.0 0.0) (`SplineComponent.GetLocationAndTangentAtSplinePoint` (`self.PathSpline`) (+ _index 1) "World") (0.0 0.0 0.0) true) ; manipulate the spline mesh to render\nbetween the current spline point and\nthe next spline point
        )))))

(fn `FindClosestObjective`
  (returns (outClosestObjective :type "Actor Object Reference"))
  (locals (_LocalDistToClosestObjective :type "Float (double-precision)") (_LocalClosestObjective :type "Actor Object Reference"))
  (set `local._LocalDistToClosestObjective` 6.45098425374317e+18) ; Set to float_max
  (for _array_element (`self.ObjectiveArray`)
    (`/Engine/EditorBlueprintResources/StandardMacros.IsValid` _array_element ; Check to make sure that objective is valid
      (:`Is Valid`
        (bind _pathlength (`NavigationSystemV1.GetPathLength` (`self.K2_GetActorLocation` (`GameplayStatics.GetPlayerPawn` 0)) (`self.K2_GetActorLocation` _array_element) null null))
        (if (> (`local._LocalDistToClosestObjective`) _pathlength)
          (set `local._LocalDistToClosestObjective` _pathlength)
          (set `local._LocalClosestObjective` _array_element)))))
  (return (`local._LocalClosestObjective`)) ; return a ref to the closest objective\nthat we saved earlier, during our\nForEach loop
)

(fn `UserConstructionScript`)