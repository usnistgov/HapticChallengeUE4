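; Police light prop for the HapticChallenge content that animates red and blue lights.
; On BeginPlay it creates a dynamic material instance on the LightPlane mesh and starts separate red and blue timelines.
; Each timeline's curve drives both that color's emissive-style multiplier parameter on the material and the intensity of its matching light component, keeping plane and lights in sync.
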(event `self.ReceiveBeginPlay`
  (`|ExecutionSequence`
    (:`then_1`
      (bind _returnvalue (`PrimitiveComponent.CreateDynamicMaterialInstance` (`self.LightPlane`) 0 (`PrimitiveComponent.GetMaterial` (`self.LightPlane`) 0) "None"))
      (set `self.LightPlaneDynMatInst` _returnvalue))
    (:`then_2`
      (bind (_direction _affectsworld) (`Timeline|RedLightTimeline`)
        (:`Update`
          (`MaterialInstanceDynamic.SetScalarParameterValue` (`self.LightPlaneDynMatInst`) "RedMultiplier" _affectsworld)
          (`LightComponent.SetIntensity` (`self.RedLight`) (* _affectsworld 1000.0)))))
    (:`then_3`
      (bind (_direction_2 _affectsworld_2) (`Timeline|BlueLightTimeline`)
        (:`Update`
          (`MaterialInstanceDynamic.SetScalarParameterValue` (`self.LightPlaneDynMatInst`) "BlueMultiplier" _affectsworld_2)
          (`LightComponent.SetIntensity` (`self.BlueLight`) (* _affectsworld_2 1000.0)))))))

(fn `UserConstructionScript`)