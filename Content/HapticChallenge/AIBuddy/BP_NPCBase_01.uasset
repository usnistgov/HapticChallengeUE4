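; Base NPC character for the AI Buddy in HapticChallenge, with movement that depends on its Standing, Crouching or Prone stance.
; Every Tick, it selects the movement data for the current stance and copies base walk speed and rotation rate into CharacterMovement.
; On BeginPlay, it attaches an arrow to the mesh's spine_03 socket, keeping world rotation, as a debug marker for the mesh centerpoint.
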(event `self.ReceiveBeginPlay`
  ;[1 0 0] For debug visualization of mesh centerpoint
  (`SceneComponent.K2_AttachToComponent` (`self.Arrow1`) (`self.Mesh`) "spine_03_socket" "SnapToTarget" "KeepWorld" "SnapToTarget" true))

(event `self.ReceiveTick`
  (params (DeltaSeconds :type "Float (single-precision)"))
  (bind (_basewalkspeed _rotationrate) (break `/Game/HapticChallenge/AIBuddy/S_NPCStanceMovementData` (select `/Game/HapticChallenge/AIBuddy/E_NPCStance` (`self.stance`) :`NewEnumerator0` (`self.standingMovementData`) :`NewEnumerator1` (`self.crouchingMovementData`) :`NewEnumerator2` (`self.proneMovementData`))))
  ;[0 0 0] Modify variables in the CharacterMovement component based on what stance this character is currently in
  (`|ExecutionSequence`
    (:`then_0`
      (set `CharacterMovementComponent.MaxWalkSpeed` _basewalkspeed (`self.CharacterMovement`)))
    (:`then_1`
      (set `CharacterMovementComponent.RotationRate` _rotationrate (`self.CharacterMovement`)))))

(fn `UserConstructionScript`)