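; AI controller for the VR buddy NPC, which follows the player, clears their view and matches their crouch.
; On the player's teleport event, it teleports the NPC to the start point and walks it toward the destination.
; Tick sidesteps it after it lingers in the camera's view cone and updates its look-at target.
; Stance combines headset-height crouch detection, ignored while looking down, with scripted crouch/prone events; player-driven prone is disconnected.
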(event `self.ReceiveBeginPlay`
  (`parent.ReceiveBeginPlay`)
  (`|ExecutionSequence`
    (:`then_0`
      ;[0 0 0] Set playerRef
      (bind _asbp_motion_controller_pawn_child_01 (cast `/Game/HapticChallenge/VR/BP_MotionControllerPawnChild_01` (`GameplayStatics.GetPlayerPawn` 0)))
      (set `self.playerRef` _asbp_motion_controller_pawn_child_01))
    (:`then_1`
      ;[0 0 0] Set pawnCharacterRef
      (bind _asbp_npcbase_01 (cast `/Game/HapticChallenge/AIBuddy/BP_NPCBase_01` (`self.K2_GetPawn`)))
      (set `self.pawnCharacterRef` _asbp_npcbase_01))
    (:`then_2`
      ;[0 0 0] Bind FollowPlayer event to EventOnExecuteTeleport in the player BP
      (add `/Game/HapticChallenge/VR/BP_MotionControllerPawnChild_01.OnTeleportEvent` (`self.playerRef`) (delegate `FollowPlayer`)))))

(event `FollowPlayer`
  (params (inStartLocation :type "Vector Structure") (inEndLocation :type "Vector Structure"))
  (bind _returnvalue (+ inStartLocation (`KismetMathLibrary.MakeVector` 0.0 0.0 (`CapsuleComponent.GetScaledCapsuleHalfHeight` (`Character.CapsuleComponent` (`self.pawnCharacterRef`))))))
  (bind (_returnvalue_roll _returnvalue_pitch _returnvalue_yaw) (`KismetMathLibrary.BreakRotator` (`KismetMathLibrary.FindLookAtRotation` _returnvalue inEndLocation)))
  ;[0 0 0] Logic to make AI Buddy follow player (called by MotionControllerPawn)
  (`self.StopMovement` self)
  (`self.K2_TeleportTo` (`self.K2_GetPawn`) _returnvalue (`KismetMathLibrary.MakeRotator` 0.0 0.0 _returnvalue_yaw))
  (`self.SetControlRotTowardsPlayer`)
  (`self.MoveToLocation` self inEndLocation 150.0 true true false true null true))

(event `self.ReceiveTick`
  (params (DeltaSeconds :type "Float (single-precision)"))
  (bind _playerref (`self.playerRef`))
  (bind _camera (`/Game/HapticChallenge/Core/VRTemplate/VirtualRealityBP/MotionControllerPawn.Camera` (`self.playerRef`)))
  (bind _camera_2 (`/Game/HapticChallenge/Core/VRTemplate/VirtualRealityBP/MotionControllerPawn.Camera` (`self.playerRef`)))
  (bind (_returnvalue_x _returnvalue_y _returnvalue_z) (`KismetMathLibrary.BreakVector` (`SceneComponent.K2_GetComponentLocation` (`/Game/HapticChallenge/Core/VRTemplate/VirtualRealityBP/MotionControllerPawn.Camera` _playerref))))
  (bind (_returnvalue_x_2 _returnvalue_y_2 _returnvalue_z_2) (`KismetMathLibrary.BreakVector` (`SceneComponent.K2_GetComponentLocation` (`Actor.RootComponent` _playerref))))
  (bind (_returnvalue_roll _returnvalue_pitch) (`KismetMathLibrary.BreakRotator` (`SceneComponent.K2_GetComponentRotation` (`/Game/HapticChallenge/Core/VRTemplate/VirtualRealityBP/MotionControllerPawn.Camera` (`self.playerRef`)))))
  (bind _returnvalue (`SceneComponent.K2_GetComponentLocation` _camera))
  (`parent.ReceiveTick` DeltaSeconds)
  (`|ExecutionSequence`
    (:`then_0`
      ;[0 0 0] Function calls to handle moving out of the player's view if necessary
      (bind (_outdoesobstructplayerview _outmovetoplayersleft) (`self.CheckIfObstructPlayerView`))
      (if _outdoesobstructplayerview
        (`self.MoveOutOfPlayerView` _outmovetoplayersleft)))
    (:`then_1`
      ;[1 0 0] Debug visualization of movement targets when NPC tries to move out of player view
      (if (`self.ShowDebug`)
        (`KismetSystemLibrary.DrawDebugString` (+ (* (`SceneComponent.GetForwardVector` _camera) 50.0) _returnvalue) (`KismetStringLibrary.Conv_RotatorToString` (`KismetMathLibrary.NormalizedDeltaRotator` (`SceneComponent.K2_GetComponentRotation` _camera) (`KismetMathLibrary.FindLookAtRotation` _returnvalue (`SceneComponent.GetSocketLocation` (`Character.Mesh` (`self.pawnCharacterRef`)) "spine_03_socket")))) null (struct :`R` 1.0 :`B` 0.316846 :`A` 1.0))))
    (:`then_2`
      ;[0 0 0] Set LookAtTargetLoc
      (set `self.LookAtTargetLoc` (`SceneComponent.K2_GetComponentLocation` (`/Game/HapticChallenge/Core/VRTemplate/VirtualRealityBP/MotionControllerPawn.Camera` (`self.playerRef`)))))
    (:`then_3`
      ;[1 0 0] Debug visualization of whatever is plugged in to "text"
      (if (`self.ShowDebug`)
        (`KismetSystemLibrary.DrawDebugString` (+ (+ (* (`SceneComponent.GetForwardVector` _camera_2) 50.0) (`SceneComponent.K2_GetComponentLocation` _camera_2)) (0.0 0.0 2.0)) (`|GetEnumeratorNameAsString` (`/Game/HapticChallenge/AIBuddy/BP_NPCBase_01.stance` (`self.pawnCharacterRef`))) null (struct :`R` 1.0 :`B` 0.316846 :`A` 1.0))))
    (:`then_4`
      ;[0 0 0] Determine currentPlayerHeadHeight and set isCrouchingWithPlayer and isProneWithPlayer accordingly
      (set `self.currentPlayerHeadHeight` (`KismetMathLibrary.Abs` (- (`KismetMathLibrary.Abs` _returnvalue_z) (`KismetMathLibrary.Abs` _returnvalue_z_2))))
      (if (>= _returnvalue_pitch -40.0)
        (bind _asbp_game_instance_vr (cast `/Game/HapticChallenge/Core/Framework/BP_GameInstanceVR` (`GameplayStatics.GetGameInstance`)))
        (if (< (`self.currentPlayerHeadHeight`) (* (`/Game/HapticChallenge/Core/Framework/BP_GameInstanceVR.UserEyeHeight` _asbp_game_instance_vr) 0.75))
          (if (not (< (`self.currentPlayerHeadHeight`) (* (`self.playerStandingHeight`) 0.5)))
            (set `self.isCrouchingWithPlayer` true)
            (set `self.isProneWithPlayer` false))
          (else
            (set `self.isCrouchingWithPlayer` false)
            (set `self.isProneWithPlayer` false)))))
    (:`then_5`
      ;[0 0 0] Set the appropriate value for stance in the controlled pawn
      (if (`self.isProneScripted`)
        (set `/Game/HapticChallenge/AIBuddy/BP_NPCBase_01.stance` "NewEnumerator2" (`self.pawnCharacterRef`))
        (elif (`self.isProneWithPlayer`)
          (set `/Game/HapticChallenge/AIBuddy/BP_NPCBase_01.stance` "NewEnumerator2" (`self.pawnCharacterRef`))
          (elif (`self.isCrouchingScripted`)
            (set `/Game/HapticChallenge/AIBuddy/BP_NPCBase_01.stance` "NewEnumerator1" (`self.pawnCharacterRef`))
            (elif (`self.isCrouchingWithPlayer`)
              (set `/Game/HapticChallenge/AIBuddy/BP_NPCBase_01.stance` "NewEnumerator1" (`self.pawnCharacterRef`))
              (else
                (set `/Game/HapticChallenge/AIBuddy/BP_NPCBase_01.stance` "NewEnumerator0" (`self.pawnCharacterRef`))))))))))

(event `OnCrouchScripted`
  ;[0 0 0] Events called by StanceModifierVolume
  (set `self.isCrouchingScripted` true))

(event `OnUncrouchScripted`
  ;[0 0 0] Events called by StanceModifierVolume
  (set `self.isCrouchingScripted` false))

(event `OnProneScripted`
  ;[0 0 0] Events called by StanceModifierVolume
  (set `self.isProneScripted` true))

(event `OnUnproneScripted`
  ;[0 0 0] Events called by StanceModifierVolume
  (set `self.isProneScripted` false))

(fn `CheckIfObstructPlayerView`
  (returns (outDoesObstructPlayerView :type Boolean) (outMoveToPlayersLeft :type Boolean))
  (bind _camera (`/Game/HapticChallenge/Core/VRTemplate/VirtualRealityBP/MotionControllerPawn.Camera` (`self.playerRef`)))
  (bind _ascharacter (cast `Character` (`self.K2_GetPawn`)))
  (bind (_returnvalue_roll _returnvalue_pitch _returnvalue_yaw) (`KismetMathLibrary.BreakRotator` (`KismetMathLibrary.NormalizedDeltaRotator` (`SceneComponent.K2_GetComponentRotation` _camera) (`KismetMathLibrary.FindLookAtRotation` (`SceneComponent.K2_GetComponentLocation` _camera) (`SceneComponent.GetSocketLocation` (`Character.Mesh` _ascharacter) "CenterOfMassSocket")))))
  (if (and (`KismetMathLibrary.InRange_FloatFloat` _returnvalue_pitch -10.0 15.0) (`KismetMathLibrary.InRange_FloatFloat` _returnvalue_yaw -10.0 10.0))
    (set `self.obstructPlayerViewTimeIncr` (+ (`self.obstructPlayerViewTimeIncr`) (`GameplayStatics.GetWorldDeltaSeconds`)))
    (if (>= (`self.obstructPlayerViewTimeIncr`) (`self.obstructPlayerViewTimeMax`))
      (set `self.obstructPlayerViewTimeIncr` 0.0)
      (return true (>= _returnvalue_yaw 0.0))
      (else
        _))
    (else
      (set `self.obstructPlayerViewTimeIncr` 0.0)))
  (return false false))

(fn `MoveOutOfPlayerView`
  (params (inMoveToPlayersLeft :type Boolean))
  (bind _returnvalue (`self.K2_GetActorLocation` (`self.K2_GetPawn`)))
  (bind _camera (`/Game/HapticChallenge/Core/VRTemplate/VirtualRealityBP/MotionControllerPawn.Camera` (`self.playerRef`)))
  (bind (_returnvalue_x _returnvalue_y) (`KismetMathLibrary.BreakVector` (+ (`SceneComponent.K2_GetComponentLocation` _camera) (* (`KismetMathLibrary.GreaterGreater_VectorRotator` (`SceneComponent.GetForwardVector` _camera) (`KismetMathLibrary.MakeRotator` 0.0 0.0 (* (`KismetMathLibrary.SelectFloat` -1.0 1.0 inMoveToPlayersLeft) (`self.angleToMoveOutOfPlayerView`)))) (`KismetMathLibrary.VSize` (- (`SceneComponent.K2_GetComponentLocation` (`/Game/HapticChallenge/Core/VRTemplate/VirtualRealityBP/MotionControllerPawn.Camera` (`self.playerRef`))) _returnvalue))))))
  (bind _returnvalue_2 (`KismetMathLibrary.MakeVector` _returnvalue_x _returnvalue_y (.z _returnvalue)))
  (`self.StopMovement` self)
  (`self.SetControlRotTowardsPlayer`)
  (`self.MoveToLocation` self _returnvalue_2 -1.0 false true false true null true)
  (if (`self.ShowDebug`)
    (`KismetSystemLibrary.PrintString` "MOVING MOVING MOVING MOVING MOVING" true true (struct :`R` 1.0 :`G` 0.047313 :`A` 1.0))
    (`KismetSystemLibrary.DrawDebugSphere` _returnvalue_2 20.0 12 (struct :`R` 1.0 :`B` 0.806108 :`A` 1.0) 9999999999.0 2.0)))

(fn `SetControlRotTowardsPlayer`
  (bind (_returnvalue_roll _returnvalue_pitch) (`KismetMathLibrary.BreakRotator` (`self.K2_GetActorRotation` (`self.K2_GetPawn`))))
  (bind _ascharacter (cast `Character` (`self.K2_GetPawn`)))
  (bind _returnvalue (`SceneComponent.GetSocketLocation` (`Character.Mesh` _ascharacter) "spine_03_socket"))
  (bind (_returnvalue_roll_2 _returnvalue_pitch_2 _returnvalue_yaw) (`KismetMathLibrary.BreakRotator` (`KismetMathLibrary.FindLookAtRotation` (`SceneComponent.K2_GetComponentLocation` (`/Game/HapticChallenge/Core/VRTemplate/VirtualRealityBP/MotionControllerPawn.Camera` (`self.playerRef`))) _returnvalue)))
  (`self.SetControlRotation` self (`KismetMathLibrary.MakeRotator` _returnvalue_roll _returnvalue_pitch _returnvalue_yaw))
  (if (`self.ShowDebug`)
    (`KismetSystemLibrary.DrawDebugArrow` _returnvalue (+ _returnvalue (* (`KismetMathLibrary.GetForwardVector` (`KismetMathLibrary.MakeRotator` _returnvalue_roll _returnvalue_pitch _returnvalue_yaw)) 10.0)) 5.0 (struct :`R` 0.16292 :`B` 1.0 :`A` 1.0) 999999.0 1.0)))

(fn `UserConstructionScript`)