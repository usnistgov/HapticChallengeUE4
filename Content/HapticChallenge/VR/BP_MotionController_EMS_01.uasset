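; VR motion controller that lets the player pick up and place EMS gear at gear place points.
; A looping timer finds the closest eligible place point overlapping the grab sphere and moves the hover highlight to it.
; With gear held, only points of matching gear type qualify; empty-handed, only points with removable gear do.
; Grab and release delegate pickup and drop to the hovered point and track the attached actor.
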(event `self.ReceiveBeginPlay`
  (`|ExecutionSequence`
    (:`then_1`
      (`parent.ReceiveBeginPlay`)
      (`|ExecutionSequence`
        (:`then_0`
          (`KismetSystemLibrary.K2_SetTimerDelegate` (delegate `CheckForPlacePoints`) 0.1 true))))))

(event `CheckForPlacePoints`
  (`|ExecutionSequence`
    (:`then_0`
      (bind (_outpointfound _outclosestpoint) (`self.GetNearbyPlacePoints`))
      (bind _output_get (set `self.NewNearbyPlacePoint` _outclosestpoint))
      (if (`KismetSystemLibrary.IsValid` _output_get)
        (if (not (== (`self.NewNearbyPlacePoint`) (`self.OldNearbyPlacePoint`)))
          (message `/Game/HapticChallenge/Core/VRTemplate/VirtualRealityBP/PickupActorInterface.StartHover` (`self.NewNearbyPlacePoint`))
          (if (`KismetSystemLibrary.IsValid` (`self.OldNearbyPlacePoint`)) :!label _label
            (message `/Game/HapticChallenge/Core/VRTemplate/VirtualRealityBP/PickupActorInterface.EndHover` (`self.OldNearbyPlacePoint`))))
        (else
          (goto _label))))
    (:`then_1`
      (set `self.OldNearbyPlacePoint` (`self.NewNearbyPlacePoint`)))))

(event `self.ReceiveTick`
  (params (DeltaSeconds :type "Float (single-precision)"))
  (`parent.ReceiveTick` DeltaSeconds))

(event `self.GrabActor`
  (set `self.bWantsToGrip` true)
  (if (and (not (`KismetSystemLibrary.IsValid` (`self.AttachedActor`))) (`KismetSystemLibrary.IsValid` (`self.NewNearbyPlacePoint`)) (not (`GameplayStatics.IsGamePaused`)))
    (bind _outpickedupactor (message `/Game/HapticChallenge/Core/VRTemplate/VirtualRealityBP/PickupActorInterface.Pickup` (`self.NewNearbyPlacePoint`) (`self.HandMesh`)))
    (`/Engine/EditorBlueprintResources/StandardMacros.IsValid` _outpickedupactor
      (:`Is Valid`
        (set `self.AttachedActor` _outpickedupactor)))))

(event `self.ReleaseActor`
  (set `self.bWantsToGrip` false)
  (if (and (`KismetSystemLibrary.IsValid` (`self.AttachedActor`)) (`KismetSystemLibrary.IsValid` (`self.NewNearbyPlacePoint`)) (not (`GameplayStatics.IsGamePaused`)))
    (bind _outsuccess (message `/Game/HapticChallenge/Core/VRTemplate/VirtualRealityBP/PickupActorInterface.Drop` (`self.NewNearbyPlacePoint`) (`self.AttachedActor`)))
    (if _outsuccess
      (set `self.AttachedActor` null))))

(fn `GetNearbyPlacePoints`
  (returns (outPointFound :type Boolean) (outClosestPoint :type "/Game/HapticChallenge/Interactables/EMSGear/placepoint/BP_GearPlacePoint_0 Object Reference"))
  (locals (closestPoint :type "Actor Object Reference") (closestDistance :type "Float (double-precision)" :default 9999.0))
  (bind _overlappingactors (`PrimitiveComponent.GetOverlappingActors` (`self.GrabSphere`) "/Game/HapticChallenge/Interactables/EMSGear/placepoint/BP_GearPlacePoint_0.BP_GearPlacePoint_0_C"))
  (if (> (`KismetArrayLibrary.Array_Length` _overlappingactors) 0)
    (for _array_element _overlappingactors
      (bind _returnvalue (`KismetMathLibrary.VSize` (- (`SceneComponent.K2_GetComponentLocation` (`self.GrabSphere`)) (`self.K2_GetActorLocation` _array_element))))
      (if (< _returnvalue (`local.closestDistance`))
        (bind _asbp_gear_place_point_0 (cast `/Game/HapticChallenge/Interactables/EMSGear/placepoint/BP_GearPlacePoint_0` _array_element))
        (if (`KismetSystemLibrary.IsValid` (`self.AttachedActor`))
          (bind _asbp_emsgear_parent (cast `/Game/HapticChallenge/Interactables/EMSGear/BP_EMSGearParent` (`self.AttachedActor`)))
          (if (== (`/Game/HapticChallenge/Interactables/EMSGear/BP_EMSGearParent.GearTpe` _asbp_emsgear_parent) (`/Game/HapticChallenge/Interactables/EMSGear/placepoint/BP_GearPlacePoint_0.GearType` _asbp_gear_place_point_0))
            (set `local.closestDistance` _returnvalue)
            (set `local.closestPoint` _array_element))
          (elif (and (`KismetSystemLibrary.IsValid` (`/Game/HapticChallenge/Interactables/EMSGear/placepoint/BP_GearPlacePoint_0.AttachedGear` _asbp_gear_place_point_0)) (not (`/Game/HapticChallenge/Interactables/EMSGear/placepoint/BP_GearPlacePoint_0.PermanentAttach` _asbp_gear_place_point_0)))
            (set `local.closestDistance` _returnvalue)
            (set `local.closestPoint` _array_element)))))
    (bind _asbp_gear_place_point_0_2 (cast `/Game/HapticChallenge/Interactables/EMSGear/placepoint/BP_GearPlacePoint_0` (`local.closestPoint`)))
    (return true _asbp_gear_place_point_0_2)
    (else
      (return false null))))

(fn `UserConstructionScript`
  (`parent.UserConstructionScript`))