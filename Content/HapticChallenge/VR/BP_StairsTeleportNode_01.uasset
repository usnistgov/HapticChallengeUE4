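; Stairs teleport node for VR in the Haptic Challenge, a child actor that stores where the player will teleport to.
; BeginPlay caches the world position of DestinationLocationObject as DestinationLocation.
; The construction script builds an arrow from ArrowSpline, placing spline meshes between points and a static mesh tip at the end.
; Arrow pieces share NodeMatInst, start hidden in game and are reparented to IconParent keeping world transforms.
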(event `self.ReceiveBeginPlay`
  (`parent.ReceiveBeginPlay`)
  ;[0 0 0] Set location that player will teleport to
  (set `self.DestinationLocation` (`SceneComponent.K2_GetComponentLocation` (`self.DestinationLocationObject`))))

(fn `UserConstructionScript`
  (bind _arrowspline (`self.ArrowSpline`))
  (bind _arrowspline_2 (`self.ArrowSpline`))
  (bind _returnvalue (`SplineComponent.GetNumberOfSplinePoints` _arrowspline))
  (`parent.UserConstructionScript`)
  ;[0 0 0] Loop through each point in the spline
  (for _index (range (+ (- (`SplineComponent.GetNumberOfSplinePoints` (`self.ArrowSpline`)) 2) 1))
    ;[0 0 0] Add arrow body meshes between each point in the spline
    (bind _returnvalue_2 (`AddComponent|NODE_AddSplineMeshComponent-0` :`bManualAttachment` true))
    (`PrimitiveComponent.SetMaterial` _returnvalue_2 0 (`self.NodeMatInst`))
    (`SceneComponent.K2_AttachToComponent` _returnvalue_2 (`self.ArrowSpline`) "None" "KeepRelative" "KeepRelative" "KeepRelative" true)
    (bind (_location _tangent) (`SplineComponent.GetLocationAndTangentAtSplinePoint` _arrowspline_2 _index "Local"))
    (bind (_location_2 _tangent_2) (`SplineComponent.GetLocationAndTangentAtSplinePoint` _arrowspline_2 (+ _index 1) "Local"))
    (`SplineMeshComponent.SetStartAndEnd` _returnvalue_2 _location _tangent _location_2 _tangent_2 true)
    (`SceneComponent.SetHiddenInGame` _returnvalue_2 true false)
    (`SceneComponent.K2_AttachToComponent` _returnvalue_2 (`self.IconParent`) "None" "KeepWorld" "KeepWorld" "KeepWorld" true))
  ;[0 0 0] Spawn pointed end cap of arrow at the last point in the spline
  (bind _returnvalue_3 (`AddComponent|NODE_AddStaticMeshComponent-0`))
  (`PrimitiveComponent.SetMaterial` _returnvalue_3 0 (`self.NodeMatInst`))
  (`SceneComponent.K2_AttachToComponent` _returnvalue_3 (`self.ArrowSpline`) "None" "KeepRelative" "KeepRelative" "KeepRelative" true)
  (`SceneComponent.K2_SetRelativeLocationAndRotation` _returnvalue_3 (`SplineComponent.GetLocationAtSplinePoint` _arrowspline _returnvalue "Local") (`SplineComponent.GetRotationAtSplinePoint` _arrowspline _returnvalue "Local") false false)
  (`SceneComponent.SetHiddenInGame` _returnvalue_3 true false)
  (`SceneComponent.K2_AttachToComponent` _returnvalue_3 (`self.IconParent`) "None" "KeepWorld" "KeepWorld" "KeepWorld" true))