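; VR motion controller child that adds teleport-node targeting to the parent's arc teleporter.
; Arc endpoint overlaps highlight visible BP_TeleportNode_01 actors through node material and parameter collection color, rumble the controller and raise the ring.
; A predicted projectile arc against static world, validated on the navmesh, snaps to the highlighted node, whose DestinationLocation becomes the teleport destination.
; It also caches the hand mesh transform for resetting.
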(event `self.ReceiveBeginPlay`
  (`|ExecutionSequence`
    (:`then_0`
      (`parent.ReceiveBeginPlay`))
    (:`then_1`
      (set `self.HandMeshTransform` (`SceneComponent.GetRelativeTransform` (`self.HandMesh`))))))

(event `self.ReceiveTick`
  (params (DeltaSeconds :type "Float (single-precision)"))
  (`parent.ReceiveTick` DeltaSeconds))

(event `self.ArcEndPoint.OnComponentBeginOverlap`
  (params (OverlappedComponent :type "PrimitiveComponent Object Reference") (OtherActor :type "Actor Object Reference") (OtherComp :type "PrimitiveComponent Object Reference") (OtherBodyIndex :type Integer) (bFromSweep :type Boolean) (SweepResult :type "HitResult Structure (by ref)"))
  (bind _asbp_teleport_node_01 (cast `/Game/HapticChallenge/VR/BP_TeleportNode_01` OtherActor))
  (`self.TrySetHighlightedNode` _asbp_teleport_node_01))

(event `self.ArcEndPoint.OnComponentEndOverlap`
  (params (OverlappedComponent :type "PrimitiveComponent Object Reference") (OtherActor :type "Actor Object Reference") (OtherComp :type "PrimitiveComponent Object Reference") (OtherBodyIndex :type Integer))
  (cast `/Game/HapticChallenge/VR/BP_TeleportNode_01` OtherActor)
  (`self.ResetHighlightedNode`))

(event `self.UpdateArcEndpoint`
  (params (NewLocation :type "Vector Structure") (ValidLocationFound :type Boolean))
  (`SceneComponent.SetVisibility` (`self.ArcEndPoint`) (and ValidLocationFound (`self.IsTeleporterActive`)) false)
  (`SceneComponent.K2_SetWorldLocation` (`self.ArcEndPoint`) NewLocation false true)
  (`SceneComponent.K2_SetWorldRotation` (`self.Arrow`) (`KismetMathLibrary.ComposeRotators` (`self.TeleportRotation`) (`KismetMathLibrary.MakeRotator` 0.0 0.0 (.yaw (`HeadMountedDisplayFunctionLibrary.GetOrientationAndPosition`)))) false false))

(fn `GetTeleportDestination`
  (returns (Location :type "Vector Structure") (Rotation :type "Rotator Structure"))
  (return (`self.TeleportDestination`) (`self.TeleportRotation`)))

(fn `ResetHandMeshTransform`
  (`SceneComponent.K2_SetRelativeTransform` (`self.HandMesh`) (`self.HandMeshTransform`) false false))

(fn `ResetHighlightedNode`
  (bind _defaultcolor (`self.DefaultColor`))
  (`|ExecutionSequence`
    (:`then_0`
      (bind _highlightednode (`self.HighlightedNode`)
        (:`then`
          (`MaterialInstanceDynamic.SetVectorParameterValue` (`/Game/HapticChallenge/VR/BP_TeleportNode_01.NodeMatInst` _highlightednode) "Color" _defaultcolor)
          (`KismetMaterialLibrary.SetVectorParameterValue` "/Game/HapticChallenge/Core/VRTemplate/VirtualRealityBP/TeleportMCP.TeleportMCP" "Color" _defaultcolor))
        (:`else`)))
    (:`then_1`
      (set `self.IsOverlapping` false))
    (:`then_2`
      (`SceneComponent.K2_SetRelativeLocation` (`self.Ring`) (0.0 0.0 0.0) false false))))

(fn `TraceTeleportDestination`
  (returns (Success :type Boolean) (TracePoints :type "Array of Vector Structure") (NavMeshLocation :type "Vector Structure") (TraceLocation :type "Vector Structure"))
  (locals (ProjectNavExtends :type "Float (double-precision)" :default 500.0))
  (bind _arcdirection (`self.ArcDirection`))
  (bind _projectnavextends (`local.ProjectNavExtends`))
  (bind (_outhit _outpathpositions _outlasttracedestination _returnvalue) (`GameplayStatics.Blueprint_PredictProjectilePath_ByObjectType` (`SceneComponent.K2_GetComponentLocation` _arcdirection) (* (`SceneComponent.GetForwardVector` _arcdirection) (`self.TeleportLaunchVelocity`)) true 0.0 (`|MakeArray` "ObjectTypeQuery1" :!type "EObjectTypeQuery Enum") false (`|MakeArray` self :!type "Actor Object Reference") "None" 0.0 30.0)) ; Simulate throwing a projectile (including gravity) to find a teleport location.
  (bind (_bblockinghit _binitialoverlap _time _distance _location) (`GameplayStatics.BreakHitResult` _outhit))
  (bind (_projectedlocation _returnvalue_2) (`NavigationSystemV1.K2_ProjectPointToNavigation` (`NavigationSystemV1.GetNavigationSystem`) _location null null (`KismetMathLibrary.MakeVector` _projectnavextends _projectnavextends _projectnavextends)))
  (bind _returnvalue_3 (and _returnvalue _returnvalue_2))
  (if _returnvalue_3
    (if (`self.IsOverlapping`)
      (return _returnvalue_3 _outpathpositions (`self.K2_GetActorLocation` (`self.HighlightedNode`)) _location)
      (else
        _)))
  (return _returnvalue_3 _outpathpositions _projectedlocation _location))

(fn `TrySetHighlightedNode`
  (params (inNewNode :type "/Game/HapticChallenge/VR/BP_TeleportNode_01 Object Reference"))
  (bind _highlightedcolor (`self.HighlightedColor`))
  (if (not (`/Game/HapticChallenge/VR/BP_TeleportNode_01.NodeHidden` inNewNode))
    (`|ExecutionSequence`
      (:`then_0`
        (set `self.HighlightedNode` inNewNode))
      (:`then_1`
        (set `self.TeleportDestination` (`/Game/HapticChallenge/VR/BP_TeleportNode_01.DestinationLocation` (`self.HighlightedNode`))))
      (:`then_2`
        (set `self.IsOverlapping` true))
      (:`then_3`
        (`MaterialInstanceDynamic.SetVectorParameterValue` (`/Game/HapticChallenge/VR/BP_TeleportNode_01.NodeMatInst` (`self.HighlightedNode`)) "Color" _highlightedcolor)
        (`KismetMaterialLibrary.SetVectorParameterValue` "/Game/HapticChallenge/Core/VRTemplate/VirtualRealityBP/TeleportMCP.TeleportMCP" "Color" _highlightedcolor))
      (:`then_4`
        (`self.RumbleController` 0.3))
      (:`then_5`
        (`SceneComponent.K2_SetRelativeLocation` (`self.Ring`) (0.0 0.0 40.0) false false)))))

(fn `UserConstructionScript`
  (`parent.UserConstructionScript`))