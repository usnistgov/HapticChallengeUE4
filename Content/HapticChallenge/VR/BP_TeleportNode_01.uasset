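; VR teleport node actor that marks a fixed destination for the player, caching its own location at BeginPlay.
; Show and hide events toggle the icon hierarchy and track its hidden state, with showing allowed only while the node is enabled.
; Enabling or disabling switches the trigger volume's collision without changing icon visibility.
; The construction script creates and stores a dynamic material instance for the node mesh.
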(event `self.ReceiveBeginPlay`
  ;[0 0 0] Set location that player will teleport to
  (set `self.DestinationLocation` (`self.K2_GetActorLocation`)))

(event `ShowNode`
  (if (`self.NodeEnabled`)
    (`SceneComponent.SetHiddenInGame` (`self.IconParent`) false true)
    (set `self.NodeHidden` false)))

(event `HideNode`
  (`SceneComponent.SetHiddenInGame` (`self.IconParent`) true true)
  (set `self.NodeHidden` true))

(event `SetNodeEnabled`
  (params (inNodeEnabled :type Boolean))
  (bind _output_get (set `self.NodeEnabled` inNodeEnabled))
  (`PrimitiveComponent.SetCollisionEnabled` (`self.TriggerVolume`) (select `bool` _output_get :`false` "NoCollision" :`true` "QueryAndPhysics" :!type "ECollisionEnabled Enum")))

(fn `UserConstructionScript`
  (bind _nodemesh (`self.NodeMesh`))
  (bind _returnvalue (`PrimitiveComponent.CreateDynamicMaterialInstance` _nodemesh 0 (`PrimitiveComponent.GetMaterial` _nodemesh 0) "None"))
  (set `self.NodeMatInst` _returnvalue))