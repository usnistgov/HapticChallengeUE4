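; Level start and end marker for the Haptic Challenge that places the player and triggers scenario completion.
; On BeginPlay it moves the player pawn to the SpawnPoint transform.
; When exit is allowed, the motion controller pawn's collision sphere entering TriggerVolume shows the scenario-complete menu once, after a short delay.
; The delay does not recheck the overlap, a gap noted in a TODO about players teleporting away.
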(event `self.ReceiveBeginPlay`
  (bind (_returnvalue_location _returnvalue_rotation) (`KismetMathLibrary.BreakTransform` (`SceneComponent.K2_GetComponentToWorld` (`self.SpawnPoint`))))
  ;[0 0 0] Spawn player at the correct spawn point for this scenario
  (`self.K2_SetActorLocationAndRotation` (`GameplayStatics.GetPlayerPawn` 0) _returnvalue_location _returnvalue_rotation false false))

(event `self.TriggerVolume.OnComponentHit`
  (params (HitComponent :type "PrimitiveComponent Object Reference") (OtherActor :type "Actor Object Reference") (OtherComp :type "PrimitiveComponent Object Reference") (NormalImpulse :type "Vector Structure") (Hit :type "HitResult Structure (by ref)")))

(event `self.TriggerVolume.OnComponentBeginOverlap`
  (params (OverlappedComponent :type "PrimitiveComponent Object Reference") (OtherActor :type "Actor Object Reference") (OtherComp :type "PrimitiveComponent Object Reference") (OtherBodyIndex :type Integer) (bFromSweep :type Boolean) (SweepResult :type "HitResult Structure (by ref)"))
  (if (`self.AllowExitFromLevel`)
    (bind _asbp_motion_controller_pawn_child_01 (cast `/Game/HapticChallenge/VR/BP_MotionControllerPawnChild_01` OtherActor))
    (if (== (`/Game/HapticChallenge/VR/BP_MotionControllerPawnChild_01.SphereCollision` _asbp_motion_controller_pawn_child_01) OtherComp)
      ;[1 1 1] TODO develop solution that works even if player teleports to exit then teleports away before the delay completes
      (`KismetSystemLibrary.Delay` 0.5)
      (`/Engine/EditorBlueprintResources/StandardMacros.DoOnce` false
        (:`Completed`
          (`/Game/HapticChallenge/VR/BP_MotionControllerPawnChild_01.ShowScenarioCompleteMenu` _asbp_motion_controller_pawn_child_01))))))

(fn `UserConstructionScript`)