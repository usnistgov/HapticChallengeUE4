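; EMS victim actor for the haptic challenge that accepts medical gear and reports its vital readings to an EMS tablet.
; The construction script points five child-actor gear place points (left/right oximeter, ECG, left/right BP cuff) at body mesh sockets.
; BeginPlay toggles their collision from IsInteractable.
; BindPlacementPointEventsToTablet binds their attach events to tablet display calls, with blood pressure going to DisplayBPCuffError and debug text.
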(event `self.ReceiveBeginPlay`
  (`self.SetPlacePointsInteractable` (`self.IsInteractable`)))

(event `BindPlacementPointEventsToTablet`
  (params (inTabletWBP :type "/Game/HapticChallenge/Menus/WBP_EMSTablet Object Reference"))
  ;[0 0 0] Bind the OnAttach events in the placepoints to event listeners in the EMS Tablet
  (`|ExecutionSequence`
    (:`then_0`
      (bind _asbp_gear_place_point_0 (cast `/Game/HapticChallenge/Interactables/EMSGear/placepoint/BP_GearPlacePoint_0` (`ChildActorComponent.ChildActor` (`self.PlacePoint_Oximeter_Left`))))
      (add `/Game/HapticChallenge/Interactables/EMSGear/placepoint/BP_GearPlacePoint_0.OnAttachToPoint` _asbp_gear_place_point_0 (delegate `OximeterAttached`)))
    (:`then_1`
      (bind _asbp_gear_place_point_0_2 (cast `/Game/HapticChallenge/Interactables/EMSGear/placepoint/BP_GearPlacePoint_0` (`ChildActorComponent.ChildActor` (`self.PlacePoint_Oximeter_Right`))))
      (add `/Game/HapticChallenge/Interactables/EMSGear/placepoint/BP_GearPlacePoint_0.OnAttachToPoint` _asbp_gear_place_point_0_2 (delegate `OximeterAttached`)))
    (:`then_2`
      (bind _asbp_gear_place_point_0_3 (cast `/Game/HapticChallenge/Interactables/EMSGear/placepoint/BP_GearPlacePoint_0` (`ChildActorComponent.ChildActor` (`self.PlacePoint_ECG`))))
      (add `/Game/HapticChallenge/Interactables/EMSGear/placepoint/BP_GearPlacePoint_0.OnAttachToPoint` _asbp_gear_place_point_0_3 (delegate `ECGAttached`)))
    (:`then_3`
      (bind _asbp_gear_place_point_0_4 (cast `/Game/HapticChallenge/Interactables/EMSGear/placepoint/BP_GearPlacePoint_0` (`ChildActorComponent.ChildActor` (`self.PlacePoint_BPCuff_Left`))))
      (add `/Game/HapticChallenge/Interactables/EMSGear/placepoint/BP_GearPlacePoint_0.OnAttachToPoint` _asbp_gear_place_point_0_4 (delegate `BPCuffAttached`)))
    (:`then_4`
      (bind _asbp_gear_place_point_0_5 (cast `/Game/HapticChallenge/Interactables/EMSGear/placepoint/BP_GearPlacePoint_0` (`ChildActorComponent.ChildActor` (`self.PlacePoint_BPCuff_Right`))))
      (add `/Game/HapticChallenge/Interactables/EMSGear/placepoint/BP_GearPlacePoint_0.OnAttachToPoint` _asbp_gear_place_point_0_5 (delegate `BPCuffAttached`)))))

(event `OximeterAttached`
  ;[0 0 0] Bind the OnAttach events in the placepoints to event listeners in the EMS Tablet
  (`/Game/HapticChallenge/Menus/WBP_EMSTablet.DisplayOximeterStats` (stale `BindPlacementPointEventsToTablet` inTabletWBP) (`.SpO2_3_5469BA6343308C473FCD37BA860EECC4` (break `/Game/HapticChallenge/Interactables/EMSGear/S_EMSReadings` (`self.Readings`)))))

(event `ECGAttached`
  ;[0 0 0] Bind the OnAttach events in the placepoints to event listeners in the EMS Tablet
  (`/Game/HapticChallenge/Menus/WBP_EMSTablet.DisplayECGStats` (stale `BindPlacementPointEventsToTablet` inTabletWBP) (`.HeartRateBPM_6_D5FF648B46FDF0B4B3D170B003CA9BEC` (break `/Game/HapticChallenge/Interactables/EMSGear/S_EMSReadings` (`self.Readings`)))))

(event `BPCuffAttached`
  (bind (_spo2 _temperature _heartratebpm _bloodpressure) (break `/Game/HapticChallenge/Interactables/EMSGear/S_EMSReadings` (`self.Readings`)))
  ;[0 0 0] Bind the OnAttach events in the placepoints to event listeners in the EMS Tablet
  (`/Game/HapticChallenge/Menus/WBP_EMSTablet.DisplayBPCuffError` (stale `BindPlacementPointEventsToTablet` inTabletWBP) _bloodpressure)
  (`TextRenderComponent.K2_SetText` (`self.DebugTextRender2`) (`KismetTextLibrary.Conv_IntToText` _bloodpressure)))

(fn `SetPlacePointsInteractable`
  (params (inIsInteractable :type Boolean))
  (for _array_element (`|MakeArray` (`self.PlacePoint_BPCuff_Right`) (`self.PlacePoint_BPCuff_Left`) (`self.PlacePoint_ECG`) (`self.PlacePoint_Oximeter_Right`) (`self.PlacePoint_Oximeter_Left`))
    (bind _asbp_gear_place_point_0 (cast `/Game/HapticChallenge/Interactables/EMSGear/placepoint/BP_GearPlacePoint_0` (`ChildActorComponent.ChildActor` _array_element)))
    (`self.SetActorEnableCollision` _asbp_gear_place_point_0 inIsInteractable)))

(fn `UserConstructionScript`
  (`|ExecutionSequence`
    (:`then_0`
      (bind _asbp_gear_place_point_0 (cast `/Game/HapticChallenge/Interactables/EMSGear/placepoint/BP_GearPlacePoint_0` (`ChildActorComponent.ChildActor` (`self.PlacePoint_Oximeter_Right`))))
      (set `/Game/HapticChallenge/Interactables/EMSGear/placepoint/BP_GearPlacePoint_0.ComponentToAttachTo` (`self.BodyMesh`) _asbp_gear_place_point_0)
      (set `/Game/HapticChallenge/Interactables/EMSGear/placepoint/BP_GearPlacePoint_0.SocketNameToAttachTo` "Socket_Oximeter_Right" _asbp_gear_place_point_0))
    (:`then_1`
      (bind _asbp_gear_place_point_0_2 (cast `/Game/HapticChallenge/Interactables/EMSGear/placepoint/BP_GearPlacePoint_0` (`ChildActorComponent.ChildActor` (`self.PlacePoint_Oximeter_Left`))))
      (set `/Game/HapticChallenge/Interactables/EMSGear/placepoint/BP_GearPlacePoint_0.ComponentToAttachTo` (`self.BodyMesh`) _asbp_gear_place_point_0_2)
      (set `/Game/HapticChallenge/Interactables/EMSGear/placepoint/BP_GearPlacePoint_0.SocketNameToAttachTo` "Socket_Oximeter_Left" _asbp_gear_place_point_0_2))
    (:`then_2`
      (bind _asbp_gear_place_point_0_3 (cast `/Game/HapticChallenge/Interactables/EMSGear/placepoint/BP_GearPlacePoint_0` (`ChildActorComponent.ChildActor` (`self.PlacePoint_ECG`))))
      (set `/Game/HapticChallenge/Interactables/EMSGear/placepoint/BP_GearPlacePoint_0.ComponentToAttachTo` (`self.BodyMesh`) _asbp_gear_place_point_0_3)
      (set `/Game/HapticChallenge/Interactables/EMSGear/placepoint/BP_GearPlacePoint_0.SocketNameToAttachTo` "Socket_ECG" _asbp_gear_place_point_0_3))
    (:`then_3`
      (bind _asbp_gear_place_point_0_4 (cast `/Game/HapticChallenge/Interactables/EMSGear/placepoint/BP_GearPlacePoint_0` (`ChildActorComponent.ChildActor` (`self.PlacePoint_BPCuff_Right`))))
      (set `/Game/HapticChallenge/Interactables/EMSGear/placepoint/BP_GearPlacePoint_0.ComponentToAttachTo` (`self.BodyMesh`) _asbp_gear_place_point_0_4)
      (set `/Game/HapticChallenge/Interactables/EMSGear/placepoint/BP_GearPlacePoint_0.SocketNameToAttachTo` "Socket_BPCuff_Right" _asbp_gear_place_point_0_4))
    (:`then_4`
      (bind _asbp_gear_place_point_0_5 (cast `/Game/HapticChallenge/Interactables/EMSGear/placepoint/BP_GearPlacePoint_0` (`ChildActorComponent.ChildActor` (`self.PlacePoint_BPCuff_Left`))))
      (set `/Game/HapticChallenge/Interactables/EMSGear/placepoint/BP_GearPlacePoint_0.ComponentToAttachTo` (`self.BodyMesh`) _asbp_gear_place_point_0_5)
      (set `/Game/HapticChallenge/Interactables/EMSGear/placepoint/BP_GearPlacePoint_0.SocketNameToAttachTo` "Socket_BPCuff_Left" _asbp_gear_place_point_0_5))
    (:`then_5`
      (`TextRenderComponent.K2_SetText` (`self.DebugTextRender`) (`self.DebugText`)))))