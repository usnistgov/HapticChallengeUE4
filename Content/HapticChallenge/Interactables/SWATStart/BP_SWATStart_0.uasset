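; VR start station for the SWAT challenge that begins play once the player stands in position and aims the gun at the starting zone.
; A looping timer checks camera overlap with the player volume and line-traces from the gun muzzle to the gun volume.
; While ready, Tick drives a countdown with audio, text and progress bar, resetting when readiness is lost.
; On completion it fires OnStartEvent, beeps, briefly shows start text, then destroys itself.
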(event `self.ReceiveBeginPlay`
  (`|ExecutionSequence`
    (:`then_1`
      ;[0 0 0] Get and store a ref to the player
      (bind _asbp_motion_controller_pawn_swat_01 (cast `/Game/HapticChallenge/VR/BP_MotionControllerPawn_SWAT_01` (`GameplayStatics.GetPlayerPawn` 0)))
      (set `self.PlayerRef` _asbp_motion_controller_pawn_swat_01))
    (:`then_3`
      (`KismetSystemLibrary.K2_SetTimerDelegate` (delegate `CheckIfPlayerReady`) 0.01 true))))

(event `CheckIfPlayerReady`
  (if (`PrimitiveComponent.IsOverlappingComponent` (`/Game/HapticChallenge/VR/BP_MotionControllerPawn_SWAT_01.CameraCollision` (`self.PlayerRef`)) (`self.PlayerTriggerVolume`))
    (bind _outispointingatstartingzone (`self.IsGunPointingAtStartingZone`))
    (set `self.PlayerIsReady` _outispointingatstartingzone)))

(event `self.ReceiveTick`
  (params (DeltaSeconds :type "Float (single-precision)"))
  (bind _returnvalue (- (`self.StartDelay`) (`self.StartDelayIterator`)))
  (`/Engine/EditorBlueprintResources/StandardMacros.Gate` false :!label _label
    (:`Exit`
      (if (`self.PlayerIsReady`)
        (`|ExecutionSequence`
          (:`then_0`
            (`/Engine/EditorBlueprintResources/StandardMacros.DoOnce` false :!label _label_2
              (:`Completed`
                (`AudioComponent.Play` (`self.AudioSource`) 0.0))))
          (:`then_1`
            (`SceneComponent.SetHiddenInGame` (`self.TimerParent`) false true)
            (set `self.StartDelayIterator` (+ (`self.StartDelayIterator`) (`GameplayStatics.GetWorldDeltaSeconds`)))
            (if (>= (`self.StartDelayIterator`) (`self.StartDelay`))
              (`SceneComponent.SetHiddenInGame` (`self.PlayerTriggerVolume`) true true)
              (`SceneComponent.SetHiddenInGame` (`self.GunTriggerVolume`) true true)
              (`SceneComponent.SetHiddenInGame` (`self.TimerProgressBar`) true true)
              (`SceneComponent.SetHiddenInGame` (`self.PromptText`) true true)
              (`self.OnStartEvent`)
              (`|ExecutionSequence`
                (:`then_0`
                  (goto _label :!via `Close`))
                (:`then_1`
                  (`AudioComponent.SetSound` (`self.AudioSource`) "/Game/HapticChallenge/Audio/SoundWaves/A_ui_timer_beep_high_01.A_ui_timer_beep_high_01")
                  (`AudioComponent.Play` (`self.AudioSource`) 0.0))
                (:`then_2`
                  (`TextRenderComponent.K2_SetText` (`self.TimerText`) (`self.TextToDisplayOnStart`))
                  (`KismetSystemLibrary.Delay` 1.0)
                  (`SceneComponent.SetHiddenInGame` (`self.TimerText`) true true)
                  (clear `self.OnStartEvent`)
                  (`self.K2_DestroyActor`)))
              (else
                (`TextRenderComponent.K2_SetText` (`self.TimerText`) (`KismetTextLibrary.Conv_DoubleToText` _returnvalue "ToPositiveInfinity" false true 1 1 0 0))
                (`MeshComponent.SetScalarParameterValueOnMaterials` (`self.TimerProgressBar`) "ProgressAmount" (`KismetMathLibrary.Fraction` _returnvalue))))))
        (else
          (`|ExecutionSequence`
            (:`then_0`
              (`AudioComponent.Stop` (`self.AudioSource`))
              (goto _label_2 :!via `Reset`))
            (:`then_1`
              (set `self.StartDelayIterator` 0.0)
              (`SceneComponent.SetHiddenInGame` (`self.TimerParent`) true true))))))))

(fn `IsGunPointingAtStartingZone`
  (returns (outIsPointingAtStartingZone :type Boolean))
  (bind _playerref (`self.PlayerRef`))
  (bind _bulletspawnpoint (`/Game/HapticChallenge/Interactables/Guns/BP_FirearmTwoHanded_01.BulletSpawnPoint` (`self.GunRef`)))
  (bind _returnvalue (`SceneComponent.K2_GetComponentLocation` _bulletspawnpoint))
  (bind _returnvalue_2 (`SceneComponent.GetForwardVector` _bulletspawnpoint))
  (bind (_outhit _returnvalue_3) (`KismetSystemLibrary.LineTraceSingleForObjects` (+ _returnvalue (* _returnvalue_2 -50.0)) (+ _returnvalue (* _returnvalue_2 300.0)) (`|MakeArray` "ObjectTypeQuery2" :!type "EObjectTypeQuery Enum") false (`|MakeArray` (`self.GunRef`) _playerref (`/Game/HapticChallenge/Core/VRTemplate/VirtualRealityBP/MotionControllerPawn.LeftController` _playerref) (`/Game/HapticChallenge/Core/VRTemplate/VirtualRealityBP/MotionControllerPawn.RightController` _playerref) null :!type "Actor Object Reference") "None" false))
  (if _returnvalue_3
    (return (== (`self.GunTriggerVolume`) (`.HitComponent` (`GameplayStatics.BreakHitResult` _outhit))))
    (else
      (return false))))

(fn `UserConstructionScript`
  (`TextRenderComponent.K2_SetText` (`self.PromptText`) (`self.TextToDisplayOnPrompt`)))