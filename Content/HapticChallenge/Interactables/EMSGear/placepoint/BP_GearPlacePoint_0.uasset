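; Placement point for EMS gear (oximeter, ECG, blood pressure cuff) that accepts only gear of its own type, optionally as a permanent attachment.
; Construction picks the preview mesh, which stays hidden until hover outlines it through custom depth.
; Drop attaches and hides the gear, showing the preview mesh instead; Pickup moves non-permanent gear to a type-specific socket.
; Both play per-type sounds, and RecentlyPickedUp blocks re-dropping until hover ends.
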(event `self.ReceiveBeginPlay`
  (`|ExecutionSequence`
    (:`then_0`
      (if (and (!= (`self.SocketNameToAttachTo`) "None") (`KismetSystemLibrary.IsValid` (`self.ComponentToAttachTo`)))
        (`SceneComponent.K2_AttachToComponent` (`self.GearMesh`) (`self.ComponentToAttachTo`) (`self.SocketNameToAttachTo`) "SnapToTarget" "SnapToTarget" "SnapToTarget" true)))
    (:`then_1`
      (`PrimitiveComponent.SetRenderCustomDepth` (`self.GearMesh`) false)
      (`PrimitiveComponent.SetRenderInMainPass` (`self.GearMesh`) false))))

(event `/Game/HapticChallenge/Core/VRTemplate/VirtualRealityBP/PickupActorInterface.StartHover`
  (`PrimitiveComponent.SetRenderCustomDepth` (`self.GearMesh`) true))

(event `/Game/HapticChallenge/Core/VRTemplate/VirtualRealityBP/PickupActorInterface.EndHover`
  (`PrimitiveComponent.SetRenderCustomDepth` (`self.GearMesh`) false)
  (set `self.RecentlyPickedUp` false))

(fn `Drop`
  (params (InActorBeingDropped :type "Actor Object Reference"))
  (returns (OutSuccess :type Boolean))
  (locals (LocalActorBeingDropped :type "/Game/HapticChallenge/Interactables/EMSGear/BP_EMSGearParent Object Reference"))
  (if (not (`self.RecentlyPickedUp`))
    (bind _asbp_emsgear_parent (cast `/Game/HapticChallenge/Interactables/EMSGear/BP_EMSGearParent` InActorBeingDropped))
    (bind _output_get (set `local.LocalActorBeingDropped` _asbp_emsgear_parent))
    (if (`|EnumEquality` (`/Game/HapticChallenge/Interactables/EMSGear/BP_EMSGearParent.GearTpe` _output_get) (`self.GearType`))
      (bind _returnvalue (`SceneComponent.K2_AttachToComponent` (`self.K2_GetRootComponent` (`local.LocalActorBeingDropped`)) (`self.ComponentToAttachTo`) (`self.SocketNameToAttachTo`) "SnapToTarget" "SnapToTarget" "SnapToTarget" true))
      (if _returnvalue
        (`SceneComponent.SetHiddenInGame` (`self.K2_GetRootComponent` (`local.LocalActorBeingDropped`)) true false)
        (set `self.AttachedGear` (`local.LocalActorBeingDropped`))
        (`PrimitiveComponent.SetRenderCustomDepth` (`self.GearMesh`) false)
        (`PrimitiveComponent.SetRenderInMainPass` (`self.GearMesh`) true)
        (`self.OnAttachToPoint`)
        (if (`self.PermanentAttach`)
          (`AudioComponent.SetSound` (`self.Audio`) (select `/Game/HapticChallenge/Interactables/EMSGear/placepoint/E_EMSGearType` (`self.GearType`) :`NewEnumerator0` "/Game/HapticChallenge/Audio/SoundWaves/A_EMS_Oximeter_Attach.A_EMS_Oximeter_Attach" :`NewEnumerator1` "/Game/HapticChallenge/Audio/SoundWaves/A_EMS_ECG_Attach.A_EMS_ECG_Attach" :`NewEnumerator2` "/Game/HapticChallenge/Audio/SoundWaves/A_EMS_Cuff_Attach.A_EMS_Cuff_Attach" :!type "SoundBase Object Reference"))
          (else
            (`AudioComponent.SetSound` (`self.Audio`) (select `/Game/HapticChallenge/Interactables/EMSGear/placepoint/E_EMSGearType` (`self.GearType`) :`NewEnumerator0` "/Game/HapticChallenge/Audio/SoundWaves/A_EMS_Oximeter_PutDown.A_EMS_Oximeter_PutDown" :`NewEnumerator1` "/Game/HapticChallenge/Audio/SoundWaves/A_EMS_ECG_PutDown.A_EMS_ECG_PutDown" :`NewEnumerator2` "/Game/HapticChallenge/Audio/SoundWaves/A_EMS_Cuff_PutDown.A_EMS_Cuff_PutDown" :!type "SoundBase Object Reference"))))
        (`AudioComponent.Stop` (`self.Audio`))
        (`AudioComponent.Play` (`self.Audio`) 0.0)
        (return true)
        (else
          (return false)))
      (else
        (return false)))
    (else
      (return false))))

(fn `Pickup`
  (params (AttachTo :type "SceneComponent Object Reference"))
  (returns (OutPickedUpActor :type "Actor Object Reference"))
  (locals (LocalActorBeingPickedUp :type "/Game/HapticChallenge/Interactables/EMSGear/BP_EMSGearParent Object Reference"))
  (`/Engine/EditorBlueprintResources/StandardMacros.IsValid` (`self.AttachedGear`)
    (:`Is Valid`
      (if (not (`self.PermanentAttach`))
        (set `local.LocalActorBeingPickedUp` (`self.AttachedGear`)) ; Store AttachedGear in a local var so we can set AttachedGear to null but still have a ref to return at the end of this function
        (bind _returnvalue (`SceneComponent.K2_AttachToComponent` (`self.K2_GetRootComponent` (`self.AttachedGear`)) AttachTo (select `/Game/HapticChallenge/Interactables/EMSGear/placepoint/E_EMSGearType` (`self.GearType`) :`NewEnumerator0` "Socket_EMSOximeter" :`NewEnumerator1` "Socket_EMSECG" :`NewEnumerator2` "Socket_EMSBPCuff" :!type "Name") "SnapToTarget" "SnapToTarget" "KeepWorld" false))
        (if _returnvalue
          (`SceneComponent.SetHiddenInGame` (`self.K2_GetRootComponent` (`self.AttachedGear`)) false false)
          (set `self.AttachedGear` null)
          (`PrimitiveComponent.SetRenderInMainPass` (`self.GearMesh`) false)
          (`PrimitiveComponent.SetRenderCustomDepth` (`self.GearMesh`) false)
          (`self.OnDetachFromPoint`)
          (set `self.RecentlyPickedUp` true)
          (`AudioComponent.SetSound` (`self.Audio`) (select `/Game/HapticChallenge/Interactables/EMSGear/placepoint/E_EMSGearType` (`self.GearType`) :`NewEnumerator0` "/Game/HapticChallenge/Audio/SoundWaves/A_EMS_Oximeter_Pickup.A_EMS_Oximeter_Pickup" :`NewEnumerator1` "/Game/HapticChallenge/Audio/SoundWaves/A_EMS_ECG_PickUp.A_EMS_ECG_PickUp" :`NewEnumerator2` "/Game/HapticChallenge/Audio/SoundWaves/A_EMS_Cuff_PickUp.A_EMS_Cuff_PickUp" :!type "SoundBase Object Reference"))
          (`AudioComponent.Stop` (`self.Audio`))
          (`AudioComponent.Play` (`self.Audio`) 0.0)
          (return (`local.LocalActorBeingPickedUp`)))
        (else
          (return null))))
    (:`Is Not Valid`
      (return null))))

(fn `UserConstructionScript`
  (`|ExecutionSequence`
    (:`then_0`
      (set `self.ComponentToAttachTo` (`self.GearMesh`)) ; Set this so that, by default, an EMSGear that gets attached to us will be snapped to the location of PreviewMesh
    )
    (:`then_1`
      (switch `/Game/HapticChallenge/Interactables/EMSGear/placepoint/E_EMSGearType` (`self.GearType`) ; set the correct model for the mesh based on GearType
        (:`NewEnumerator0`
          (`StaticMeshComponent.SetStaticMesh` (`self.GearMesh`) "/Game/HapticChallenge/Art/EMS/SM_Finger_Sensor.SM_Finger_Sensor"))
        (:`NewEnumerator1`
          (`StaticMeshComponent.SetStaticMesh` (`self.GearMesh`) (select `bool` (`self.PermanentAttach`) :`false` "/Game/HapticChallenge/Art/EMS/SM_ECG_Cords_Detatched.SM_ECG_Cords_Detatched" :`true` "/Game/HapticChallenge/Art/EMS/SM_ECG_Cords_Attached.SM_ECG_Cords_Attached" :!type "StaticMesh Object Reference")))
        (:`NewEnumerator2`
          (`StaticMeshComponent.SetStaticMesh` (`self.GearMesh`) (select `bool` (`self.PermanentAttach`) :`false` "/Game/HapticChallenge/Art/EMS/SM_Arm_Cuff_Detached.SM_Arm_Cuff_Detached" :`true` "/Game/HapticChallenge/Art/EMS/SM_Arm_Cuff_Attached.SM_Arm_Cuff_Attached" :!type "StaticMesh Object Reference")))))))