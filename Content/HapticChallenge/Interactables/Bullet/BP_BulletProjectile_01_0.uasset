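; Bullet projectile that simulates drag, ricochet and material penetration, with optional speed-colored debug trails.
; Tick slows it using a speed-based drag coefficient curve.
; Each bounce flags a barrier hit, spawns impact effects by physical material, then rolls penetration from DT_MaterialPenetrationData using angle and speed.
; Penetration reverse-traces the exit point, subtracts energy by thickness and spawns a replacement bullet; deflections randomize direction within a speed-scaled cone.
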(event `self.ReceiveTick`
  (params (DeltaSeconds :type "Float (single-precision)"))
  (bind _returnvalue (* (`KismetMathLibrary.VSize` (`MovementComponent.Velocity` (`self.ProjectileMovementComponent`))) 0.01))
  (`self.DrawDebugTrace` (`self.LastPosition`) (`self.K2_GetActorLocation`) (`MovementComponent.Velocity` (`self.ProjectileMovementComponent`)))
  (set `self.LastPosition` (`self.K2_GetActorLocation`))
  ;[0 0 0] Calculate and set the new velocity of the bullet at each frame
  (set `MovementComponent.Velocity` (* (`MovementComponent.Velocity` (`self.ProjectileMovementComponent`)) (- 1.0 (/ (* (/ (* -0.5 _returnvalue 1.225 2.6e-05 (`CurveFloat.GetFloatValue` (`self.DragCoefficient`) _returnvalue) _returnvalue) (`self.BulletWeightKg`)) (`GameplayStatics.GetWorldDeltaSeconds`) -100.0) (`KismetMathLibrary.VSize` (`MovementComponent.Velocity` (`self.ProjectileMovementComponent`)))))) (`self.ProjectileMovementComponent`)))

(event `self.ProjectileMovementComponent.OnProjectileBounce`
  (params (ImpactResult :type "HitResult Structure (by ref)") (ImpactVelocity :type "Vector Structure (by ref)"))
  (bind (_outspawnlocation _outresultfound _outexithit) (`self.ComputeExitLocation` ImpactResult ImpactVelocity))
  (bind _outnewspeed (`self.GetNewSpeed` _outspawnlocation ImpactVelocity ImpactResult))
  (bind _returnvalue (* ImpactVelocity (/ _outnewspeed (`KismetMathLibrary.VSize` ImpactVelocity))))
  (`|ExecutionSequence`
    (:`then_0`
      ;[0 0 0] Use this variable to track if bullet has hit an intermediate barrier. If so, it will not count if it hits a target afterwards
      (`/Engine/EditorBlueprintResources/StandardMacros.DoOnce` false
        (:`Completed`
          (set `self.HasHitIntermediateBarrier` true))))
    (:`then_1`
      (`self.DrawDebugTrace` (`self.LastPosition`) (`.Location` (`GameplayStatics.BreakHitResult` ImpactResult)) ImpactVelocity))
    (:`then_2`
      (`self.PlayImpactSound` ImpactResult)
      (`self.PlaceImpactDecal` ImpactResult)
      (`self.PlaceImpactParticleEffect` ImpactResult)
      ;[0 0 0] Decide whether to penetrate
      (if (`self.DecideWhetherToPenetrate` ImpactResult ImpactVelocity)
        ;[0 0 0] Compute Exit Location
        (if _outresultfound
          ;[0 0 0] Compute New Speed
          (if (> _outnewspeed 0.0)
            (bind _returnvalue_2 (`|SpawnActorFromClass` "BP_BulletProjectile_01_0_C" (`KismetMathLibrary.MakeTransform` _outspawnlocation) "Undefined" "OverrideRootScale" null null))
            (set `MovementComponent.Velocity` _returnvalue (`/Game/HapticChallenge/Interactables/Bullet/BP_BulletProjectile_01_0.ProjectileMovementComponent` _returnvalue_2))
            (`self.VaryTrajectory` (`.ImpactNormal` (`GameplayStatics.BreakHitResult` _outexithit)) _returnvalue _returnvalue_2)
            (`self.K2_DestroyActor`)
            (else
              (`self.K2_DestroyActor`)))
          (else
            (`|ExecutionSequence`
              (:`then_0`
                (`self.DrawDebugTrace` (`.Location` (`GameplayStatics.BreakHitResult` ImpactResult)) (`self.K2_GetActorLocation`) (`MovementComponent.Velocity` (`self.ProjectileMovementComponent`))))
              (:`then_1`
                (`self.K2_DestroyActor`)))))
        (else
          (`self.VaryTrajectory` (`.Location` (`GameplayStatics.BreakHitResult` ImpactResult)) ImpactVelocity self))))))

(fn `ComputeExitLocation`
  (params (inHitResult :type "HitResult Structure") (inImpactVelocity :type "Vector Structure"))
  (returns (outSpawnLocation :type "Vector Structure") (outResultFound :type Boolean) (outExitHit :type "HitResult Structure"))
  (locals (LocalHitResult :type "HitResult Structure") (LocalImpactVelocity :type "Vector Structure") (LocalExitHit :type "HitResult Structure") (PreliminaryExitLocation :type "Vector Structure"))
  (bind (_bblockinghit _binitialoverlap _time _distance _location) (`GameplayStatics.BreakHitResult` inHitResult))
  (set `local.LocalHitResult` inHitResult)
  (set `local.LocalImpactVelocity` inImpactVelocity)
  (bind (_outhits _returnvalue) (`KismetSystemLibrary.SphereTraceMultiForObjects` (+ (* (`KismetMathLibrary.Normal` inImpactVelocity) 500.0) _location) _location (`SphereComponent.SphereRadius` (`self.CollisionComponent`)) (`|MakeArray` "ObjectTypeQuery1" "ObjectTypeQuery2" "ObjectTypeQuery3" "ObjectTypeQuery4" "ObjectTypeQuery5" "ObjectTypeQuery6" :!type "EObjectTypeQuery Enum")))
  (if _returnvalue
    (bind _returnvalue_2 (`KismetArrayLibrary.Array_LastIndex` _outhits))
    (for _index (range (+ _returnvalue_2 1))
      (bind _output (`|GetArrayItem` _outhits (- _returnvalue_2 _index)))
      (bind (_bblockinghit_2 _binitialoverlap_2 _time_2 _distance_2 _location_2 _impactpoint _normal _impactnormal _physmat _hitactor) (`GameplayStatics.BreakHitResult` _output))
      (if (== _hitactor (`.HitActor` (`GameplayStatics.BreakHitResult` (`local.LocalHitResult`))))
        (set `local.LocalExitHit` _output)
        (bind _output_get (set `local.PreliminaryExitLocation` (+ _location_2 _impactnormal)))
        (bind (_outhit _returnvalue_3) (`KismetSystemLibrary.SphereTraceSingleForObjects` _output_get (+ _output_get (`KismetMathLibrary.Normal` (`local.LocalImpactVelocity`))) (`SphereComponent.SphereRadius` (`self.CollisionComponent`)) (`|MakeArray` "ObjectTypeQuery1" "ObjectTypeQuery2" "ObjectTypeQuery3" "ObjectTypeQuery4" "ObjectTypeQuery5" "ObjectTypeQuery6" :!type "EObjectTypeQuery Enum")))
        (if _returnvalue_3
          (bind (_outspawnlocation _outresultfound _outexithit) (`self.ComputeExitLocation` _outhit (`local.LocalImpactVelocity`)))
          (return _outspawnlocation true _outexithit)
          (else
            (return (`local.PreliminaryExitLocation`) true (`local.LocalExitHit`))))))
    (return (0.0 0.0 0.0) false)
    (else
      (return (0.0 0.0 0.0) false))))

(fn `DecideWhetherToPenetrate`
  (params (inHit :type "HitResult Structure") (inImpactVelocity :type "Vector Structure"))
  (returns (outDoesPenetrate :type Boolean))
  (locals (LocalImpactAngleCoefficient :type "Float (double-precision)" :default -0.0222) (LocalImpactAngleConstant :type "Float (double-precision)" :default 1.333) (LocalVelocityCoefficient :type "Float (double-precision)" :default 0.000125) (LocalVelocityConstant :type "Float (double-precision)" :default -6.0))
  (bind (_bblockinghit _binitialoverlap _time _distance _location _impactpoint _normal _impactnormal _physmat) (`GameplayStatics.BreakHitResult` inHit))
  (bind _returnvalue (`|GetDataTableRow` "/Game/HapticChallenge/Interactables/Guns/AR-15/DT_MaterialPenetrationData.DT_MaterialPenetrationData" (`KismetStringLibrary.Conv_StringToName` (`KismetSystemLibrary.GetObjectName` _physmat)))
    (:`then`
      (`|ExecutionSequence`
        (:`then_0`
          (bind (_joulespercm _impactanglecoefficient _impactangleconstant _velocitycoefficient _velocityconstant) (break `/Game/HapticChallenge/Interactables/Bullet/S_MaterialPenetrationData` _returnvalue))
          (set `local.LocalImpactAngleCoefficient` _impactanglecoefficient))
        (:`then_1`
          (set `local.LocalImpactAngleConstant` _impactangleconstant))
        (:`then_2`
          (set `local.LocalVelocityCoefficient` _velocitycoefficient))
        (:`then_3`
          (set `local.LocalVelocityConstant` _velocityconstant))
        (:`then_4`
          (return (> (* (`KismetMathLibrary.FClamp` (+ (* (`self.GetAngleBetweenVectors` inImpactVelocity (* _impactnormal -1.0)) (`local.LocalImpactAngleCoefficient`)) (`local.LocalImpactAngleConstant`))) (`KismetMathLibrary.FClamp` (+ (* (`KismetMathLibrary.VSize` inImpactVelocity) (`local.LocalVelocityCoefficient`)) (`local.LocalVelocityConstant`)))) (`KismetMathLibrary.RandomFloatInRange` 0.0 1.0))))))
    (:`RowNotFound`
      (return (> (* (`KismetMathLibrary.FClamp` (+ (* (`self.GetAngleBetweenVectors` inImpactVelocity (* _impactnormal -1.0)) (`local.LocalImpactAngleCoefficient`)) (`local.LocalImpactAngleConstant`))) (`KismetMathLibrary.FClamp` (+ (* (`KismetMathLibrary.VSize` inImpactVelocity) (`local.LocalVelocityCoefficient`)) (`local.LocalVelocityConstant`)))) (`KismetMathLibrary.RandomFloatInRange` 0.0 1.0))))))

(fn `DrawDebugTrace`
  (params (inStart :type "Vector Structure") (inEnd :type "Vector Structure") (inVelocity :type "Vector Structure"))
  (if (`self.ShouldDrawDebugTrace`)
    (`KismetSystemLibrary.DrawDebugLine` inStart inEnd (`self.GetDebugTraceColor` inVelocity) (`self.DebugTraceDuration`))))

(fn `GetAngleBetweenVectors`
  (params (inVector1 :type "Vector Structure") (inVector2 :type "Vector Structure"))
  (returns (outAngle :type "Float (double-precision)"))
  (return (`KismetMathLibrary.DegAcos` (`KismetMathLibrary.Dot_VectorVector` (`KismetMathLibrary.Normal` inVector1) (`KismetMathLibrary.Normal` inVector2)))))

(fn `GetDebugTraceColor`
  (params (inVelocity :type "Vector Structure"))
  (returns (outColor :type "LinearColor Structure"))
  (locals (SpeedFraction :type "Float (double-precision)"))
  (bind _output_get (set `local.SpeedFraction` (/ (`KismetMathLibrary.VSize` inVelocity) (`ProjectileMovementComponent.InitialSpeed` (`self.ProjectileMovementComponent`)))))
  (if (> _output_get 0.75)
    (return (`KismetMathLibrary.LinearColorLerp` (struct :`R` 1.0 :`G` 1.0 :`A` 1.0) (struct :`R` 1.0 :`A` 1.0) (* (- (`local.SpeedFraction`) 0.75) 4.0)))
    (elif (> (`local.SpeedFraction`) 0.5)
      (return (`KismetMathLibrary.LinearColorLerp` (struct :`G` 1.0 :`A` 1.0) (struct :`R` 1.0 :`G` 1.0 :`A` 1.0) (* (- (`local.SpeedFraction`) 0.5) 4.0)))
      (elif (> (`local.SpeedFraction`) 0.25)
        (return (`KismetMathLibrary.LinearColorLerp` (struct :`B` 1.0 :`A` 1.0) (struct :`G` 1.0 :`A` 1.0) (* (- (`local.SpeedFraction`) 0.25) 4.0)))))))

(fn `GetNewSpeed`
  (params (inExitLocation :type "Vector Structure") (inImpactVelocity :type "Vector Structure") (inHit :type "HitResult Structure"))
  (returns (outNewSpeed :type "Float (double-precision)"))
  (locals (LocalJoulesPerCM :type "Float (double-precision)" :default 200.0))
  (bind (_bblockinghit _binitialoverlap _time _distance _location _impactpoint _normal _impactnormal _physmat) (`GameplayStatics.BreakHitResult` inHit))
  (bind _returnvalue (`|GetDataTableRow` "/Game/HapticChallenge/Interactables/Guns/AR-15/DT_MaterialPenetrationData.DT_MaterialPenetrationData" (`KismetStringLibrary.Conv_StringToName` (`KismetSystemLibrary.GetObjectName` _physmat)))
    (:`then`
      (set `local.LocalJoulesPerCM` (`.JoulesPerCM_2_105449454E57BFC558B2CF9AFFD2242F` (break `/Game/HapticChallenge/Interactables/Bullet/S_MaterialPenetrationData` _returnvalue)))
      (return (`KismetMathLibrary.Sqrt` (/ (- (* 0.5 (`self.BulletWeightKg`) (`KismetMathLibrary.VSizeSquared` inImpactVelocity)) (* (`KismetMathLibrary.VSize` (- inExitLocation _location)) (`local.LocalJoulesPerCM`))) (* (`self.BulletWeightKg`) 0.5)))))))

(fn `PlaceImpactDecal`
  (params (inHit :type "HitResult Structure"))
  (locals (localLocation :type "Vector Structure") (localDecalToPlace :type "MaterialInstance Object Reference" :default "MaterialInstanceConstant'/Game/HapticChallenge/Art/ImpactDecals/MI_Decal_Impact_Concrete.MI_Decal_Impact_Concrete'") (LocalNormal :type "Vector Structure" :default (0.0 0.0 0.0)))
  (bind (_bblockinghit _binitialoverlap _time _distance _location _impactpoint _normal _impactnormal _physmat) (`GameplayStatics.BreakHitResult` inHit))
  (set `local.localLocation` _location)
  (set `local.LocalNormal` _normal)
  (switch `name` (`KismetStringLibrary.Conv_StringToName` (`KismetSystemLibrary.GetObjectName` _physmat))
    (:`Default`
      (set `local.localDecalToPlace` "/Game/HapticChallenge/Art/ImpactDecals/MI_Decal_Impact_Concrete.MI_Decal_Impact_Concrete" :!label _label))
    (:`PM_Concrete`
      (goto _label))
    (:`PM_Wood`
      (goto _label))
    (:`PM_Steel`
      (set `local.localDecalToPlace` "/Game/HapticChallenge/Art/ImpactDecals/MI_Decal_Impact_CarBody.MI_Decal_Impact_CarBody" :!label _label_2))
    (:`PM_CarBody`
      (goto _label_2))
    (:`PM_CarGlass`
      (goto _label))
    (:`PM_Target`
      (goto _label_2))
    (:`PM_PlasticStrong`
      (set `local.localDecalToPlace` "/Game/HapticChallenge/Art/ImpactDecals/MI_Decal_Impact_PlasticStrong.MI_Decal_Impact_PlasticStrong")))
  (bind _returnvalue (`KismetMaterialLibrary.CreateDynamicMaterialInstance` (`local.localDecalToPlace`)))
  (bind _returnvalue_2 (`MaterialInstanceDynamic.K2_GetScalarParameterValue` _returnvalue "NumImagesX"))
  (bind _returnvalue_3 (`MaterialInstanceDynamic.K2_GetScalarParameterValue` _returnvalue "NumImagesY"))
  (`MaterialInstanceDynamic.SetScalarParameterValue` _returnvalue "ImageIndexToDisplay" (`KismetMathLibrary.Conv_IntToDouble` (`KismetMathLibrary.RandomIntegerInRange` 0 (`KismetMathLibrary.FTrunc` (- (* _returnvalue_3 _returnvalue_2) 1.0)))))
  (bind _returnvalue_4 (`GameplayStatics.SpawnDecalAtLocation` _returnvalue (5.0 10.0 10.0) (`local.localLocation`) (`KismetMathLibrary.ComposeRotators` (`KismetMathLibrary.MakeRotator` (`KismetMathLibrary.RandomFloatInRange` 0.0 360.0)) (`KismetMathLibrary.Conv_VectorToRotator` (* (`local.LocalNormal`) -1.0))) 60.0))
  (`DecalComponent.SetFadeScreenSize` _returnvalue_4 1e-06))

(fn `PlaceImpactParticleEffect`
  (params (inHit :type "HitResult Structure"))
  (locals (localParticleEffectToPlace :type "ParticleSystem Object Reference") (localLocation :type "Vector Structure"))
  (bind (_bblockinghit _binitialoverlap _time _distance _location _impactpoint _normal _impactnormal _physmat) (`GameplayStatics.BreakHitResult` inHit))
  (set `local.localLocation` _location)
  (switch `name` (`KismetStringLibrary.Conv_StringToName` (`KismetSystemLibrary.GetObjectName` _physmat))
    (:`Default`
      (set `local.localParticleEffectToPlace` "/Game/HapticChallenge/Art/Law/P_ConcreteImpact.P_ConcreteImpact" :!label _label))
    (:`PM_Concrete`
      (goto _label))
    (:`PM_Wood`
      (goto _label))
    (:`PM_Steel`
      (set `local.localParticleEffectToPlace` "/Game/HapticChallenge/Art/Law/P_MetalImpact.P_MetalImpact" :!label _label_2))
    (:`PM_CarBody`
      (goto _label_2))
    (:`PM_CarGlass`
      (goto _label))
    (:`PM_Target`
      (goto _label_2))
    (:`PM_PlasticStrong`
      (goto _label)))
  (`GameplayStatics.SpawnEmitterAtLocation` (`local.localParticleEffectToPlace`) (`local.localLocation`)))

(fn `PlayImpactSound`
  (params (inHit :type "HitResult Structure"))
  (locals (localSoundToPlay :type "SoundBase Object Reference" :default "SoundCue'/Game/HapticChallenge/Audio/SoundCues/A_gun_impact_concrete_Cue.A_gun_impact_concrete_Cue'") (localLocation :type "Vector Structure"))
  (bind (_bblockinghit _binitialoverlap _time _distance _location _impactpoint _normal _impactnormal _physmat) (`GameplayStatics.BreakHitResult` inHit))
  (set `local.localLocation` _location)
  (switch `name` (`KismetStringLibrary.Conv_StringToName` (`KismetSystemLibrary.GetObjectName` _physmat))
    (:`Default`
      (set `local.localSoundToPlay` "/Game/HapticChallenge/Audio/SoundCues/A_gun_impact_concrete_Cue.A_gun_impact_concrete_Cue"))
    (:`PM_Concrete`
      (set `local.localSoundToPlay` "/Game/HapticChallenge/Audio/SoundCues/A_gun_impact_concrete_Cue.A_gun_impact_concrete_Cue" :!label _label))
    (:`PM_Wood`
      (goto _label))
    (:`PM_Steel`
      (set `local.localSoundToPlay` "/Game/HapticChallenge/Audio/SoundCues/A_gun_impact_carbody_Cue.A_gun_impact_carbody_Cue" :!label _label_2))
    (:`PM_CarBody`
      (goto _label_2))
    (:`PM_CarGlass`
      (set `local.localSoundToPlay` "/Game/HapticChallenge/Audio/SoundCues/A_gun_impact_carglass_Cue.A_gun_impact_carglass_Cue"))
    (:`PM_Target`
      (set `local.localSoundToPlay` "/Game/HapticChallenge/Audio/SoundWaves/A_gun_impact_target_01.A_gun_impact_target_01"))
    (:`PM_PlasticStrong`
      (set `local.localSoundToPlay` "/Game/HapticChallenge/Audio/SoundCues/A_gun_impact_plasticstrong_Cue.A_gun_impact_plasticstrong_Cue")))
  (`GameplayStatics.PlaySoundAtLocation` (`local.localSoundToPlay`) (`local.localLocation`) (struct) 1.0 1.0 0.0 "/Game/HapticChallenge/Audio/Attenuation/ATT_gun_impact_default.ATT_gun_impact_default" null null))

(fn `UserConstructionScript`
  (set `self.LastPosition` (`self.K2_GetActorLocation`)))

(fn `VaryTrajectory`
  (params (inSurfaceNormal :type "Vector Structure") (inImpactVelocity :type "Vector Structure") (inProjectile :type "/Game/HapticChallenge/Interactables/Bullet/BP_BulletProjectile_01_0 Object Reference"))
  (locals (InitialAnswer :type "Vector Structure"))
  (bind _projectilemovementcomponent (`/Game/HapticChallenge/Interactables/Bullet/BP_BulletProjectile_01_0.ProjectileMovementComponent` inProjectile))
  (bind _velocity (`MovementComponent.Velocity` _projectilemovementcomponent))
  (bind _output_get (set `local.InitialAnswer` (* (`KismetMathLibrary.RandomUnitVectorInConeInRadians` _velocity (`KismetMathLibrary.MapRangeClamped` (`KismetMathLibrary.VSize` inImpactVelocity) 3000.0 10000.0 0.0 0.349)) (`KismetMathLibrary.VSize` _velocity))))
  (bind _outangle (`self.GetAngleBetweenVectors` inSurfaceNormal _output_get))
  (if (>= _outangle 90.0)
    ;[0 0 0] If the new velocity points back into the hit object, rotate it back to less than 90 deg away from the surface
    (set `MovementComponent.Velocity` (`KismetMathLibrary.GreaterGreater_VectorRotator` (`local.InitialAnswer`) (* (`KismetMathLibrary.NormalizedDeltaRotator` (`KismetMathLibrary.MakeRotFromX` inSurfaceNormal) (`KismetMathLibrary.MakeRotFromX` (`local.InitialAnswer`))) (- 1.0 (/ 89.0 _outangle)))) _projectilemovementcomponent)
    (return)
    (else
      (set `MovementComponent.Velocity` (`local.InitialAnswer`) _projectilemovementcomponent)
      (return))))