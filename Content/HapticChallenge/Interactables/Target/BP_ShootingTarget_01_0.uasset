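; Shooting range target that stands static or slides, swings or leans into view, optionally presenting and hiding itself automatically.
; Bullet hits that skipped intermediate barriers count toward neutralization, which fires an event and hides the target.
; Each counted impact plays a reaction timeline, a sound delayed by speed of sound and a random-image decal.
; The construction script positions pivots and engagement spheres, previews movement and shows range in yards from PlayerStart.
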(event `self.ReceiveBeginPlay`
  (`|ExecutionSequence`
    (:`then_0`
      ;[0 0 0] If target doesn't start out presented, then make it invisible
      (if (not (`self.CanBeShot`))
        (`SceneComponent.SetHiddenInGame` (`self.TargetMesh`) true false)))
    (:`then_1`
      ;[0 0 0] If target is supposed to present automatically, then call PresentTarget()
      (if (`self.PresentAutomatically`)
        (`self.PresentTarget`)))))

(event `self.ReceiveTick`
  (params (DeltaSeconds :type "Float (single-precision)")))

(event `self.ReceiveHit`
  (params (MyComp :type "PrimitiveComponent Object Reference") (Other :type "Actor Object Reference") (OtherComp :type "PrimitiveComponent Object Reference") (bSelfMoved :type Boolean) (HitLocation :type "Vector Structure") (HitNormal :type "Vector Structure") (NormalImpulse :type "Vector Structure") (Hit :type "HitResult Structure (by ref)"))
  (bind (_bblockinghit _binitialoverlap _time _distance _location _impactpoint _normal) (`GameplayStatics.BreakHitResult` Hit))
  (if (`self.CanBeShot`)
    (bind _asbp_bullet_projectile_01_0 (cast `/Game/HapticChallenge/Interactables/Bullet/BP_BulletProjectile_01_0` Other))
    (`/Game/HapticChallenge/Interactables/Bullet/BP_BulletProjectile_01_0.DrawDebugTrace` _asbp_bullet_projectile_01_0 (`/Game/HapticChallenge/Interactables/Bullet/BP_BulletProjectile_01_0.LastPosition` _asbp_bullet_projectile_01_0) HitLocation (`self.GetVelocity` _asbp_bullet_projectile_01_0))
    (if (`/Game/HapticChallenge/Interactables/Bullet/BP_BulletProjectile_01_0.HasHitIntermediateBarrier` _asbp_bullet_projectile_01_0)
      (`self.K2_DestroyActor` _asbp_bullet_projectile_01_0)
      (else
        (`self.K2_DestroyActor` _asbp_bullet_projectile_01_0)
        (`|ExecutionSequence`
          (:`then_0`
            ;[0 0 0] Increment HitsOnTarget
            (if (!= (`self.HitsRequiredToNeutralize`) -1)
              (`/Engine/EditorBlueprintResources/StandardMacros.IncrementInt` (`self.HitsOnTarget`)
                (:`  `
                  ;[0 0 0] If target has been hit enough to neutralize it, call OnTargetNeutralized event, then call HideTarget
                  (if (>= (`self.HitsOnTarget`) (`self.HitsRequiredToNeutralize`))
                    (`/Engine/EditorBlueprintResources/StandardMacros.DoOnce` false :!label _label
                      (:`Completed`
                        (`self.OnTargetNeutralized`)
                        (`KismetSystemLibrary.Delay` (`self.DelayAfterNeutralization`))
                        (`self.HideTarget`))))))))
          (:`then_1`
            ;[0 0 0] Play impact animation on target
            (bind (_direction _targetmeshrelativerotation) (`Timeline|BulletImpactAnimationTimeline` :!via `PlayFromStart`)
              (:`Update`
                (`SceneComponent.K2_SetRelativeRotation` (`self.TargetMesh`) (`KismetMathLibrary.MakeRotator` (.x _targetmeshrelativerotation) (.y _targetmeshrelativerotation) (.z _targetmeshrelativerotation)) false false))))
          (:`then_2`
            ;[0 0 0] Play impact sound after a delay to account for the time it takes sound to travel from the target to the player's ear
            (`KismetSystemLibrary.Delay` (/ (`KismetMathLibrary.VSize` (- (`self.K2_GetActorLocation` (`GameplayStatics.GetPlayerPawn` 0)) (`self.K2_GetActorLocation`))) 34300.0))
            (`GameplayStatics.PlaySoundAtLocation` "/Game/HapticChallenge/Audio/SoundWaves/A_gun_impact_target_01.A_gun_impact_target_01" (`self.K2_GetActorLocation`) (struct) 2.0 1.0 0.0 "/Game/HapticChallenge/Audio/Attenuation/ATT_gun_impact_target.ATT_gun_impact_target" null null))
          (:`then_3`
            ;[0 0 0] Spawn Impact Decal
            (bind _returnvalue (`KismetMaterialLibrary.CreateDynamicMaterialInstance` "/Game/HapticChallenge/Art/ImpactDecals/MI_Decal_Impact_Target.MI_Decal_Impact_Target"))
            (bind _returnvalue_2 (`MaterialInstanceDynamic.K2_GetScalarParameterValue` _returnvalue "NumImagesX"))
            (bind _returnvalue_3 (`MaterialInstanceDynamic.K2_GetScalarParameterValue` _returnvalue "NumImagesY"))
            (`MaterialInstanceDynamic.SetScalarParameterValue` _returnvalue "ImageIndexToDisplay" (`KismetMathLibrary.RandomFloatInRange` 0.0 (- (* _returnvalue_3 _returnvalue_2) 1.0)))
            (bind _returnvalue_4 (`GameplayStatics.SpawnDecalAttached` _returnvalue (1.0 10.0 10.0) (`self.TargetMesh`) "None" _location (`KismetMathLibrary.ComposeRotators` (`KismetMathLibrary.MakeRotator` (`KismetMathLibrary.RandomFloatInRange` 0.0 360.0)) (`KismetMathLibrary.Conv_VectorToRotator` (* _normal -1.0))) "KeepWorldPosition"))
            (`DecalComponent.SetFadeScreenSize` _returnvalue_4 1e-06)))))))

(event `ResetOnTargetNeutralized`
  ;[0 0 0] If target has been hit enough to neutralize it, call OnTargetNeutralized event, then call HideTarget
  (goto _label :!via `Reset`))

(event `EngageTarget`
  (`self.OnTargetEngaged`))

(event `PresentTarget`
  (`SceneComponent.SetHiddenInGame` (`self.TargetMesh`) false false) ; unhide target mesh
  (set `self.CanBeShot` true)
  (`|ExecutionSequence`
    (:`then_0`
      (goto _label_3 :!via `Reset`))
    (:`then_1`
      (`PrimitiveComponent.SetCollisionEnabled` (`self.EngagementImpactSphere`) "QueryAndPhysics")
      (`self.OnTargetPresent`)
      (bind (_direction _movementcoefficient) (`Timeline|TargetMovementTimeline` :!via `PlayFromStart` :!label _label_2)
        (:`Update`
          (`self.UpdateMovementAnimation` _movementcoefficient))
        (:`Finished`
          (switch `ETimelineDirection` _direction
            (:`Forward`
              ;[0 0 0] If HideAutomatically, wait for the specified delay then call HideTarget
              (if (`self.HideAutomatically`)
                (`KismetSystemLibrary.Delay` (`self.HideAutomaticallyDelay`))
                (`self.HideTarget`)))
            (:`Backward`
              (`SceneComponent.SetHiddenInGame` (`self.TargetMesh`) true false)
              (set `self.CanBeShot` false)
              (`PrimitiveComponent.SetCollisionEnabled` (`self.EngagementImpactSphere`) "NoCollision")
              (set `self.HitsOnTarget` 0)
              (`self.ResetOnTargetNeutralized`)
              (`self.OnTargetHidden` self)
              ;[0 0 0] If PresentAutomatically, wait for the specified delay then call PresentTarget again
              (if (`self.PresentAutomatically`)
                (`KismetSystemLibrary.Delay` (`self.PresentAutomaticallyDelay`))
                (`self.PresentTarget`)))))))))

(event `HideTarget`
  (`/Engine/EditorBlueprintResources/StandardMacros.DoOnce` true :!label _label_3 ; keep hide functionality from being called twice
    (:`Completed`
      (goto _label_2 :!via `Reverse`))))

(fn `SetHideAutomatically`
  (params (inHideAutomatically :type Boolean))
  (set `self.HideAutomatically` inHideAutomatically))

(fn `SetPresentAutomatically`
  (params (inPresentAutomatically :type Boolean))
  (set `self.PresentAutomatically` inPresentAutomatically))

(fn `UpdateMovementAnimation`
  (params (inMovementCoefficient :type "Float (double-precision)"))
  (switch `/Game/HapticChallenge/Interactables/Target/E_TargetMovementType` (`self.TargetMovementType`)
    (:`NewEnumerator1`
      (switch `/Game/HapticChallenge/Interactables/Target/E_TargetMovementDirection` (`self.TargetMovementDirection`)
        (:`NewEnumerator0`
          (`SceneComponent.K2_SetRelativeLocation` (`self.TargetSlideParent`) (`KismetMathLibrary.MakeVector` (* (`self.TargetCmToSlide`) inMovementCoefficient)) false false))
        (:`NewEnumerator1`
          (`SceneComponent.K2_SetRelativeLocation` (`self.TargetSlideParent`) (`KismetMathLibrary.MakeVector` (* (* (`self.TargetCmToSlide`) inMovementCoefficient) -1.0)) false false))
        (:`NewEnumerator3`
          (`SceneComponent.K2_SetRelativeLocation` (`self.TargetSlideParent`) (`KismetMathLibrary.MakeVector` 0.0 0.0 (* (`self.TargetCmToSlide`) inMovementCoefficient)) false false))))
    (:`NewEnumerator2`
      (switch `/Game/HapticChallenge/Interactables/Target/E_TargetMovementDirection` (`self.TargetMovementDirection`)
        (:`NewEnumerator0`
          (`SceneComponent.K2_SetRelativeRotation` (`self.TargetPivotParentLeft`) (`KismetMathLibrary.MakeRotator` 0.0 0.0 (* (`self.TargetDegreesToRotate`) inMovementCoefficient)) false false))
        (:`NewEnumerator1`
          (`SceneComponent.K2_SetRelativeRotation` (`self.TargetPivotParentRight`) (`KismetMathLibrary.MakeRotator` 0.0 0.0 (* (* (`self.TargetDegreesToRotate`) inMovementCoefficient) -1.0)) false false))
        (:`NewEnumerator3`
          (`SceneComponent.K2_SetRelativeRotation` (`self.TargetPivotParentLeft`) (`KismetMathLibrary.MakeRotator` (* (`self.TargetDegreesToRotate`) inMovementCoefficient)) false false))))
    (:`NewEnumerator3`
      (switch `/Game/HapticChallenge/Interactables/Target/E_TargetMovementDirection` (`self.TargetMovementDirection`)
        (:`NewEnumerator0`
          (`SceneComponent.K2_SetRelativeRotation` (`self.TargetPivotParentRight`) (`KismetMathLibrary.MakeRotator` 0.0 (* (* (`self.TargetDegreesToRotate`) inMovementCoefficient) -1.0)) false false))
        (:`NewEnumerator1`
          (`SceneComponent.K2_SetRelativeRotation` (`self.TargetPivotParentLeft`) (`KismetMathLibrary.MakeRotator` 0.0 (* (`self.TargetDegreesToRotate`) inMovementCoefficient)) false false))))))

(fn `UserConstructionScript`
  (bind _targetmesh (`self.TargetMesh`))
  (bind _targetmesh_2 (`self.TargetMesh`))
  (bind _targetmesh_3 (`self.TargetMesh`))
  (bind _targetmovementtype (`self.TargetMovementType`))
  (bind _targetmesh_4 (`self.TargetMesh`))
  (bind (_min _max) (`StaticMeshComponent.GetLocalBounds` (`self.TargetMesh`)))
  (bind (_min_2 _max_2) (`StaticMeshComponent.GetLocalBounds` _targetmesh_2))
  (bind (_min_3 _max_3) (`StaticMeshComponent.GetLocalBounds` _targetmesh_4))
  (bind _x (.x _max))
  (`|ExecutionSequence`
    (:`then_0`
      ;[0 0 0] Set both target meshes to be the user specified model
      (`StaticMeshComponent.SetStaticMesh` (`self.TargetMesh`) (`self.TargetMeshModel`))
      (`StaticMeshComponent.SetStaticMesh` (`self.PreviewTargetMesh`) (`self.TargetMeshModel`)))
    (:`then_1`
      ;[0 0 0] Build array of engagement vis spheres
      (set `self.EngagementSphereArray` (`|MakeArray` (`self.EngagementVisSphere_00`) (`self.EngagementVisSphere_01`) (`self.EngagementVisSphere_02`) (`self.EngagementVisSphere_03`))))
    (:`then_2`
      ;[0 0 0] Set the locations of the four engagement vis spheres to be at the four corners of the front of the target
      (`|ExecutionSequence`
        (:`then_0`
          (`SceneComponent.K2_SetWorldLocation` (`self.EngagementVisSphere_00`) (+ (`SceneComponent.K2_GetComponentLocation` _targetmesh_3) (`KismetMathLibrary.GreaterGreater_VectorRotator` (`StaticMeshComponent.GetLocalBounds` _targetmesh_3) (`SceneComponent.K2_GetComponentRotation` _targetmesh_3))) false false))
        (:`then_1`
          (`SceneComponent.K2_SetWorldLocation` (`self.EngagementVisSphere_01`) (+ (`SceneComponent.K2_GetComponentLocation` _targetmesh) (`KismetMathLibrary.GreaterGreater_VectorRotator` (`.Max` (`StaticMeshComponent.GetLocalBounds` _targetmesh)) (`SceneComponent.K2_GetComponentRotation` _targetmesh))) false false))
        (:`then_2`
          (`SceneComponent.K2_SetWorldLocation` (`self.EngagementVisSphere_02`) (+ (`SceneComponent.K2_GetComponentLocation` _targetmesh_4) (`KismetMathLibrary.GreaterGreater_VectorRotator` (`KismetMathLibrary.MakeVector` (.x _min_3) (.y _max_3) (.z _max_3)) (`SceneComponent.K2_GetComponentRotation` _targetmesh_4))) false false))
        (:`then_3`
          (`SceneComponent.K2_SetWorldLocation` (`self.EngagementVisSphere_03`) (+ (`SceneComponent.K2_GetComponentLocation` _targetmesh_2) (`KismetMathLibrary.GreaterGreater_VectorRotator` (`KismetMathLibrary.MakeVector` (.x _max_2) (.y _min_2) (.z _min_2)) (`SceneComponent.K2_GetComponentRotation` _targetmesh_2))) false false))))
    (:`then_3`
      ;[0 0 0] Set preview target be be visible in case we set it to be invisible previously
      (`SceneComponent.SetVisibility` (`self.PreviewTargetMesh`) true false))
    (:`then_4`
      ;[0 0 0] Update range display above target
      (bind _outactors (`GameplayStatics.GetAllActorsOfClass` "/Script/Engine.PlayerStart"))
      (`TextRenderComponent.K2_SetText` (`self.PreviewRangeText`) (`KismetTextLibrary.Conv_DoubleToText` (* (`KismetMathLibrary.VSize` (- (`self.K2_GetActorLocation`) (`self.K2_GetActorLocation` (`|GetArrayItem` _outactors)))) 0.010936) "HalfToEven" false true 1 324 2)))
    (:`then_5`
      ;[0 0 0] Static targets will never have CanBeShot set to true via their movement, so set it true here
      (set `self.CanBeShot` (select `/Game/HapticChallenge/Interactables/Target/E_TargetMovementType` _targetmovementtype :`NewEnumerator0` true))
      (`PrimitiveComponent.SetCollisionEnabled` (`self.EngagementImpactSphere`) (select `/Game/HapticChallenge/Interactables/Target/E_TargetMovementType` _targetmovementtype :`NewEnumerator0` "QueryAndPhysics" :`NewEnumerator1` "NoCollision" :`NewEnumerator2` "NoCollision" :`NewEnumerator3` "NoCollision" :!type "ECollisionEnabled Enum")))
    (:`then_6`
      ;[0 0 0] Adjust location of target & pivot points, and their respective preview components
      (`SceneComponent.K2_SetRelativeLocation` (`self.TargetPivotParentLeft`) _min false false)
      (`SceneComponent.K2_SetRelativeLocation` (`self.PreviewTargetPivotParentLeft`) _min false false)
      (`SceneComponent.K2_SetRelativeLocation` (`self.TargetSlideParent`) (0.0 0.0 0.0) false false)
      (`SceneComponent.K2_SetRelativeLocation` (`self.PreviewTargetSlideParent`) (0.0 0.0 0.0) false false)
      (`SceneComponent.K2_SetRelativeLocation` (`self.PreviewTargetPivotParentRight`) (`KismetMathLibrary.MakeVector` (* _x 2.0)) false false)
      (`SceneComponent.K2_SetRelativeLocation` (`self.TargetPivotParentRight`) (`KismetMathLibrary.MakeVector` (* _x 2.0)) false false)
      (`SceneComponent.K2_SetRelativeLocation` (`self.TargetMesh`) (`KismetMathLibrary.MakeVector` (* _x -1.0)) false false)
      (`SceneComponent.K2_SetRelativeLocation` (`self.PreviewTargetMesh`) (`KismetMathLibrary.MakeVector` (* _x -1.0)) false false))
    (:`then_7`
      ;[0 0 0] Update target movement preview
      (switch `/Game/HapticChallenge/Interactables/Target/E_TargetMovementType` (`self.TargetMovementType`)
        (:`NewEnumerator0`
          (set `self.TargetMovementDirection` "NewEnumerator2")
          (`SceneComponent.SetVisibility` (`self.PreviewTargetMesh`) false false)
          (set `self.HitsRequiredToNeutralize` -1))
        (:`NewEnumerator1`
          (switch `/Game/HapticChallenge/Interactables/Target/E_TargetMovementDirection` (`self.TargetMovementDirection`)
            (:`NewEnumerator0`
              (`SceneComponent.K2_SetRelativeLocation` (`self.PreviewTargetSlideParent`) (`KismetMathLibrary.MakeVector` (`self.TargetCmToSlide`)) false false))
            (:`NewEnumerator1`
              (`SceneComponent.K2_SetRelativeLocation` (`self.PreviewTargetSlideParent`) (`KismetMathLibrary.MakeVector` (* (`self.TargetCmToSlide`) -1.0)) false false))
            (:`NewEnumerator3`
              (`SceneComponent.K2_SetRelativeLocation` (`self.PreviewTargetSlideParent`) (`KismetMathLibrary.MakeVector` 0.0 0.0 (`self.TargetCmToSlide`)) false false))))
        (:`NewEnumerator2`
          (switch `/Game/HapticChallenge/Interactables/Target/E_TargetMovementDirection` (`self.TargetMovementDirection`)
            (:`NewEnumerator0`
              (`SceneComponent.K2_SetRelativeRotation` (`self.PreviewTargetPivotParentLeft`) (`KismetMathLibrary.MakeRotator` 0.0 0.0 (`self.TargetDegreesToRotate`)) false false))
            (:`NewEnumerator1`
              (`SceneComponent.K2_SetRelativeRotation` (`self.PreviewTargetPivotParentRight`) (`KismetMathLibrary.MakeRotator` 0.0 0.0 (* (`self.TargetDegreesToRotate`) -1.0)) false false))
            (:`NewEnumerator3`
              (`SceneComponent.K2_SetRelativeRotation` (`self.PreviewTargetPivotParentLeft`) (`KismetMathLibrary.MakeRotator` (`self.TargetDegreesToRotate`)) false false))))
        (:`NewEnumerator3`
          (switch `/Game/HapticChallenge/Interactables/Target/E_TargetMovementDirection` (`self.TargetMovementDirection`)
            (:`NewEnumerator0`
              (`SceneComponent.K2_SetRelativeRotation` (`self.PreviewTargetPivotParentRight`) (`KismetMathLibrary.MakeRotator` 0.0 (* (`self.TargetDegreesToRotate`) -1.0)) false false))
            (:`NewEnumerator1`
              (`SceneComponent.K2_SetRelativeRotation` (`self.PreviewTargetPivotParentLeft`) (`KismetMathLibrary.MakeRotator` 0.0 (`self.TargetDegreesToRotate`)) false false))))))))